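; Per-player usable button that forwards use, release, cancel, completion and radial menu events to dispatchers through ROS events, gated by DispatchReplication flags.
; Optionally opens a custom radial menu on use or completion, with anti-spam briefly disabling the use collision.
; Collision is enabled only on the owning client, since other clients otherwise hit it despite owner-only visibility.
; When the owner's overlap ends, it hides the menu and the server destroys it.
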(event `Event On Use`
  (params (Pawn :type "INSSoldier Object Reference"))
  ;[0 0.1862 0.7917] The dispatchers
  (bind _output_get (set `self.Pawn` Pawn))
  (if (`|GetArrayItem` (`self.DispatchReplication`))
    (`self.Event On Use ROS` _output_get)
    ;[0.3192 1 0.2543] AntiSpam.
    (`|ExecutionSequence`
      (:`then_0`
        (if (and (`self.antiSpam`) (== (`self.UseTime`) 0.0))
          ;;[1 0 0.9765] Disables usable collision response, for Anti Spam Timeout duration.
          (`self.Set Local Collision Response` "ECR_Ignore" :!label _label)
          (`KismetSystemLibrary.Delay` (`self.AntiSpamTimeout`))
          (`self.Set Local Collision Response` "ECR_Block")))
      (:`then_1`
        ;[0.3333 0.3298 0.1868] onUse or onComplete should spawn radial?
        (if (and (== (`self.UseTime`) 0.0) (`self.createRadial`))
          (`self.MakeRadial` :!label _label_2))))))

(event `Event On Use ROS`
  (params (Pawn :type "INSSoldier Object Reference"))
  ;[0 0.1862 0.7917] The dispatchers
  (`self.OnUseDispatch` Pawn self))

(event `self.EventOnUseComplete`
  (params (Pawn :type "INSSoldier Object Reference"))
  ;[0 0.1862 0.7917] The dispatchers
  (bind _output_get (set `self.Pawn` Pawn))
  (if (`|GetArrayItem` (`self.DispatchReplication`) 1)
    (`self.Event On Use Complete ROS` _output_get)
    ;[0.3192 1 0.2543] AntiSpam.
    (`|ExecutionSequence`
      (:`then_0`
        (`|ExecutionSequence` :!label _label_3
          (:`then_0`
            (if (`self.antiSpam`)
              (goto _label)))))
      (:`then_1`
        ;[0.3333 0.3298 0.1868] onUse or onComplete should spawn radial?
        (if (and (`self.createRadial`) (> (`self.UseTime`) 0.0))
          (goto _label_2))))))

(event `Event On Use Complete ROS`
  (params (Pawn :type "INSSoldier Object Reference"))
  ;[0 0.1862 0.7917] The dispatchers
  (`self.OnUseCompleteDispatch` Pawn self))

(event `OnUseKeyReleased`
  (params (Pawn :type "INSSoldier Object Reference") (`Elapsed Time` :type "Float (double-precision)"))
  ;[0 0.1862 0.7917] The dispatchers
  (bind _output_get (set `self.Pawn` Pawn))
  (if (`|GetArrayItem` (`self.DispatchReplication`) 2)
    (`self.OnUseKeyReleased ROS` _output_get `Elapsed Time`)
    (goto _label_3)))

(event `OnUseKeyReleased ROS`
  (params (Pawn :type "INSSoldier Object Reference") (`Elapsed Time` :type "Float (double-precision)"))
  ;[0 0.1862 0.7917] The dispatchers
  (`self.OnUseReleasedDispatch` Pawn `Elapsed Time` self))

(event `self.EventOnUseCancelled`
  (params (Pawn :type "INSSoldier Object Reference"))
  ;[0 0.1862 0.7917] The dispatchers
  (bind _output_get (set `self.Pawn` Pawn))
  (if (`|GetArrayItem` (`self.DispatchReplication`) 3)
    (`self.Event On Use Cancelled ROS` _output_get)
    (goto _label_3)))

(event `Event On Use Cancelled ROS`
  (params (Pawn :type "INSSoldier Object Reference"))
  ;[0 0.1862 0.7917] The dispatchers
  (`self.OnUseCancelledDispatch` Pawn self))

(event `EventOnReceiveRadial ROS`
  (params (Direction :type "ERadialMenuDirection Enum" :default "Radial_North") (Pawn :type "INSSoldier Object Reference"))
  ;[0 0.1862 0.7917] The dispatchers
  (`self.OnRecieveRadialCommand` Direction Pawn self))

(event `EventOnHideRadial ROS`
  (params (Pawn :type "INSSoldier Object Reference"))
  ;[0 0.1862 0.7917] The dispatchers
  (`self.OnHideRadialDispatch` Pawn self))

(event `MakeRadial`
  (bind _radialmenuwidgetinstance (`self.RadialMenuWidgetInstance`))
  ;[0.1765 0.3569 0.3686] Radial Menu. Modified range computer BP
  (bind _asinsplayer_controller (cast `INSPlayerController` (`Pawn.GetController` (`self.Pawn`))))
  (if (`self.antiSpam`)
    (`self.Set Local Collision Response` "ECR_Ignore")
    (`|ExecutionSequence`
      (:`then_0`
        _)))
  (set `self.player` _asinsplayer_controller)
  (if (`self.createRadial`)
    (`/Engine/EditorBlueprintResources/StandardMacros.IsValid` _radialmenuwidgetinstance
      (:`Is Valid`
        (`INSPlayerController.ShowCustomRadial` _asinsplayer_controller _radialmenuwidgetinstance))
      (:`Is Not Valid`
        (bind _returnvalue (`INSPlayerController.CreateCustomRadial` _asinsplayer_controller (`self.Radial Menu`)))
        (bind _output_get (set `self.RadialMenuWidgetInstance` _returnvalue))
        (bind _asbp_radial_menu_custom (cast `/CustomScenario/Blueprints/BP_RadialMenuCustom` _output_get))
        (set `/CustomScenario/Blueprints/BP_RadialMenuCustom.RadialCommandsArray` (`self.RadialCommands`) _asbp_radial_menu_custom)
        (set `/CustomScenario/Blueprints/BP_RadialMenuCustom.Radial_Option_Enabled` (`self.Radial_Option_Enabled`) _asbp_radial_menu_custom)
        (add `/Game/UI/Widgets/HUD/Radial/BP_RadialMenuBase.OnSendCommand` _asbp_radial_menu_custom (delegate `OnSend`))
        (add `/CustomScenario/Blueprints/BP_RadialMenuCustom.OnHideOnOwner` _asbp_radial_menu_custom (delegate `OnHide`))
        (`/CustomScenario/Blueprints/BP_RadialMenuCustom.UpdateRangeRadialProperties` _asbp_radial_menu_custom)))))

(event `OnSend`
  (params (Direction :type "ERadialMenuDirection Enum" :default "Radial_North"))
  ;[0.1765 0.3569 0.3686] Radial Menu. Modified range computer BP
  (`self.EventOnReceiveRadial ROS` Direction (`self.Pawn`))
  (if (`self.antiSpam`) :!label _label_4
    (goto _label)))

(event `OnHide`
  ;[0.1765 0.3569 0.3686] Radial Menu. Modified range computer BP
  (`self.EventOnHideRadial ROS` (`self.Pawn`))
  (goto _label_4))

(event `self.ReceiveBeginPlay`
  ;[1 0.06519 0] BeginPlay
  (`|ExecutionSequence`
    (:`then_0`
      ;[1 0.6073 0.2872] Destroy self when the owner moves away. Runs on server and client
      ;;[0.2552 0.01196 0.01196] Avoid end overlaps as it spawns
      (`KismetSystemLibrary.Delay` 0.01)
      (goto _label_5 :!via `Open`))
    (:`then_1`
      (`self.Set Local Collision Response` "ECR_Block"))
    (:`then_2`
      ;[0.1765 0.3569 0.3686] For Radial Menu timeout
      (add `self.HideMenuDispatch` (delegate `HideMenuDispatch_Event_0`)))))

(event `HideMenuDispatch_Event_0`
  (bind _returnvalue (`Pawn.GetController` (`Actor.Instigator` (`self.GetOwner` self))))
  ;[0.1765 0.3569 0.3686] For Radial Menu timeout
  (if (`KismetSystemLibrary.IsValid` _returnvalue)
    (if (`Controller.IsLocalPlayerController` _returnvalue)
      (`KismetSystemLibrary.PrintString` "Hide" false false)
      (if (`KismetSystemLibrary.IsValid` (stale `MakeRadial` _asinsplayer_controller))
        (`INSPlayerController.HideActiveRadialWidget` (stale `MakeRadial` _asinsplayer_controller))
        (`KismetSystemLibrary.Delay` 0.04)
        (`INSBasePlayerController.ClientMessageText` (stale `MakeRadial` _asinsplayer_controller) (`KismetTextLibrary.Conv_StringToText` "Timed Out / Out of Range") "None" 5.0)))))

(event `self.Overlap.OnComponentEndOverlap`
  (params (OverlappedComponent :type "PrimitiveComponent Object Reference") (OtherActor :type "Actor Object Reference") (OtherComp :type "PrimitiveComponent Object Reference") (OtherBodyIndex :type Integer))
  ;[1 0.6073 0.2872] Destroy self when the owner moves away. Runs on server and client
  (if (and (== (`self.GetOwner` self) (`ActorComponent.GetOwner` OtherComp)) (not (`PrimitiveComponent.IsOverlappingActor` (`self.Overlap`) OtherActor)))
    (`/Engine/EditorBlueprintResources/StandardMacros.Gate` true :!label _label_5
      (:`Exit`
        (`|ExecutionSequence`
          (:`then_0`
            (`self.HideMenuDispatch`))
          (:`then_1`
            (if (`KismetSystemLibrary.IsServer`)
              (`KismetSystemLibrary.Delay` 0.05)
              (`self.K2_DestroyActor`))))))))

(event `Set Local Collision Response`
  (params (`New Response` :type "ECollisionResponse Enum" :default "ECR_Ignore"))
  (bind _instigator (`Actor.Instigator` (`self.GetOwner` self)))
  (bind _returnvalue (`Pawn.GetController` _instigator))
  ;[1 0 0.9765] Despite "only owner see=true", other clients still see other clients buttons collisions. This only enables collision on the owning client, to fix that.
  (if (`KismetSystemLibrary.IsDedicatedServer`)
    _
    (elif (`KismetSystemLibrary.IsValid` _instigator)
      (if (`KismetSystemLibrary.IsValid` _returnvalue)
        (if (`Controller.IsLocalPlayerController` _returnvalue)
          (`PrimitiveComponent.SetCollisionResponseToChannel` (`self.Use`) "ECC_GameTraceChannel4" `New Response`))))))

(fn `EventGetDynamicHintLocation`
  (params (Pawn :type "INSSoldier Object Reference") (Hit :type "HitResult Structure (by ref)"))
  (returns (ReturnValue :type "Vector Structure"))
  (return (`SceneComponent.K2_GetComponentLocation` (`self.Hint`))))

(fn `EventOnUseKeyReleased`
  (params (Pawn :type "INSSoldier Object Reference") (ElapsedTime :type "Float (double-precision)"))
  (returns (ReturnValue :type "EUseResponse Enum"))
  (`|ExecutionSequence`
    (:`then_0`
      (`self.OnUseKeyReleased` Pawn ElapsedTime))
    (:`then_1`
      (return "Handled"))))

(fn `EventTryUse`
  (params (Pawn :type "INSSoldier Object Reference") (HitResult :type "HitResult Structure (by ref)"))
  (returns (ReturnValue :type "EUseResponse Enum"))
  (`/Engine/EditorBlueprintResources/StandardMacros.IsValid` Pawn
    (:`Is Valid`
      (`self.Event On Use` Pawn)
      (return "Handled"))
    (:`Is Not Valid`
      (`KismetSystemLibrary.PrintString` "ignore")
      (return "Ignore"))))

(fn `OnRep_RadialMenuWidgetInstance`)

(fn `UserConstructionScript`)