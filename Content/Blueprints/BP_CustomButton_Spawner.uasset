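; Server-side spawner for custom interactable buttons, giving each overlapping player controller its own BP_CustomButton_PerPlayer owned by that player so presses replicate back.
; It copies its shape, use and radial menu settings onto each button and relays their use, release, cancel and radial events through its own dispatchers.
; Optional one-user mode tracks in-use state with a timeout and can hide others' buttons, while RepNotifies destroy or respawn buttons as settings change.
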(event `FromClient_OnUse`
  (params (Pawn :type "INSSoldier Object Reference") (SpawnedButton :type "Actor Object Reference"))
  ;[0.572 0 0] The binds and dispatchers
  ;;[1 1 1] onUse
  (bind _allowedout (`self.InUseStart` Pawn SpawnedButton))
  (if _allowedout
    (if (`self.DebugOn`)
      (`KismetSystemLibrary.PrintString` "OnUse"))
    (`self.OnUseDispatch` Pawn)))

(event `ReEnabled`
  (bind _overlappingactors (`PrimitiveComponent.GetOverlappingActors` (`self.OverlapSource`) "/Game/Game/Actors/Characters/BP_Character_Player.BP_Character_Player_C"))
  ;[0.1562 0.05208 0.05208] Gets overlapped actors when spawner is renabled. Works best with EnabledAffectsOverlapEvents=0
  (if (and (!= (`KismetArrayLibrary.Array_Length` _overlappingactors) 0) (`KismetSystemLibrary.IsServer`))
    (for _array_element _overlappingactors
      (`self.SpawnClientButtons` _array_element))))

(event `FromClient_OnUseComplete`
  (params (Pawn :type "INSSoldier Object Reference") (SpawnedButton :type "Actor Object Reference"))
  ;[0.572 0 0] The binds and dispatchers
  ;;[1 1 1] onUseComplete
  (bind _allowed_out (`self.InUseStop` Pawn true))
  (if _allowed_out
    (if (`self.DebugOn`)
      (`KismetSystemLibrary.PrintString` "OnUseComplete"))
    (`self.OnUseCompleteDispatch` Pawn)))

(event `SpawnClientButtons`
  (params (Actor :type "Actor Object Reference"))
  (bind _instigator (`Actor.Instigator` Actor))
  (bind _returnvalue (`Pawn.GetController` _instigator))
  (if (and (`KismetSystemLibrary.IsServer`) (`self.Enabled`) (not (`self.buttonInUse`)))
    (if (`KismetSystemLibrary.IsValid` _instigator)
      (`/Engine/EditorBlueprintResources/StandardMacros.IsValid` _returnvalue
        (:`Is Valid`
          ;[0.4471 0.06274 0.4] Checks if this controller has a spawned button already. Also prevents spawning for each overlapping child component of the player.
          (if (and (`Controller.IsPlayerController` _returnvalue) (not (`KismetArrayLibrary.Array_Contains` (`self.PlayerControllersWithSpawns`) _returnvalue)))
            (`KismetArrayLibrary.Array_Add` (`self.PlayerControllersWithSpawns`) _returnvalue)
            ;[0.1667 0.1667 0.1667] Spawn the clients button BP and give ownership to the player so they can replicate presses back to the server
            (bind _returnvalue_2 (`|SpawnActorFromClass` "/CustomScenario/Blueprints/BP_CustomButton_PerPlayer.BP_CustomButton_PerPlayer_C" (`SceneComponent.K2_GetComponentToWorld` (`self.UseSource`)) "AlwaysSpawn" "OverrideRootScale" Actor null))
            (`KismetArrayLibrary.Array_Add` (`self.SpawnedButtons`) _returnvalue_2)
            (`/Engine/EditorBlueprintResources/StandardMacros.IsValid` _returnvalue_2
              (:`Is Valid`
                (`self.SetSpawnedVariables` _returnvalue_2)
                (add `self.OnDestroyed` _returnvalue_2 (delegate `OnDestroyedButton`))
                (`|ExecutionSequence`
                  (:`then_0`
                    ;[0.572 0 0] The binds and dispatchers
                    ;;[1 1 1] onUse
                    (add `/CustomScenario/Blueprints/BP_CustomButton_PerPlayer.OnUseDispatch` _returnvalue_2 (delegate `FromClient_OnUse`)))
                  (:`then_1`
                    ;;[1 1 1] onUseComplete
                    (add `/CustomScenario/Blueprints/BP_CustomButton_PerPlayer.OnUseCompleteDispatch` _returnvalue_2 (delegate `FromClient_OnUseComplete`)))
                  (:`then_2`
                    ;;[1 1 1] onUseReleased
                    (add `/CustomScenario/Blueprints/BP_CustomButton_PerPlayer.OnUseReleasedDispatch` _returnvalue_2 (delegate `FromClient_OnUseReleased`)))
                  (:`then_3`
                    ;;[1 1 1] onUseCancelled
                    (add `/CustomScenario/Blueprints/BP_CustomButton_PerPlayer.OnUseCancelledDispatch` _returnvalue_2 (delegate `FromClient_OnUseCancelled`)))
                  (:`then_4`
                    ;;[1 1 1] onRadialSelected
                    (add `/CustomScenario/Blueprints/BP_CustomButton_PerPlayer.OnRecieveRadialCommand` _returnvalue_2 (delegate `FromClient_RecieveRadial`)))
                  (:`then_5`
                    ;;[1 1 1] onRadialHidden
                    (add `/CustomScenario/Blueprints/BP_CustomButton_PerPlayer.OnHideRadialDispatch` _returnvalue_2 (delegate `CustomEvent_0`))))))))))))

(event `self.ReceiveActorBeginOverlap`
  (params (OtherActor :type "Actor Object Reference"))
  (`self.SpawnClientButtons` OtherActor))

(event `OnDestroyedButton` :!signature `self.OnDestroyed`
  (params (DestroyedActor :type "Actor Object Reference"))
  (bind _returnvalue (`self.GetInstigatorController` (`self.GetOwner` DestroyedActor)))
  ;[0.4471 0.06274 0.4] Removes the players controller from the array so they can get a new spawned actor.
  (`KismetArrayLibrary.Array_RemoveItem` (`self.SpawnedButtons`) DestroyedActor)
  (`/Engine/EditorBlueprintResources/StandardMacros.IsValid` _returnvalue
    (:`Is Valid`
      (`KismetArrayLibrary.Array_RemoveItem` (`self.PlayerControllersWithSpawns`) _returnvalue)
      (if (and (== DestroyedActor (`self.SpawnedButton`)) (`self.buttonInUse`))
        (set `self.buttonInUse` false)))))

(event `self.ReceiveBeginPlay`
  (`|ExecutionSequence`
    (:`then_0`
      ;[1 0.1342 0.0245] Handle round restarts
      (if (`KismetSystemLibrary.IsServer`)
        _))))

(event `FromClient_OnUseReleased`
  (params (Pawn :type "INSSoldier Object Reference") (`Elapsed Time` :type "Float (double-precision)") (SpawnedButton :type "Actor Object Reference"))
  ;[0.572 0 0] The binds and dispatchers
  ;;[1 1 1] onUseReleased
  (bind _allowed_out (`self.InUseStop` Pawn))
  (if _allowed_out
    (if (`self.DebugOn`)
      (`KismetSystemLibrary.PrintString` "OnUseReleased"))
    (`self.OnUseReleasedDispatch` Pawn `Elapsed Time`)))

(event `SetSpawnedVariables`
  (params (PerPlayerBP :type "/CustomScenario/Blueprints/BP_CustomButton_PerPlayer Object Reference"))
  (bind _overlap (`/CustomScenario/Blueprints/BP_CustomButton_PerPlayer.Overlap` PerPlayerBP))
  (bind _radial_option_enabled (`self.Radial_Option_Enabled`))
  (bind _overlapsource (`self.OverlapSource`))
  ;[1 0.3515 0.05127] Run attachment and variable changes on both server and clients
  (`self.K2_AttachToActor` PerPlayerBP self "None" "KeepWorld" "KeepWorld" "KeepWorld" true)
  (`|ExecutionSequence`
    (:`then_0`
      (`SceneComponent.K2_SetRelativeTransform` (`/CustomScenario/Blueprints/BP_CustomButton_PerPlayer.Hint` PerPlayerBP) (`SceneComponent.GetRelativeTransform` (`self.HintSource`)) false false)
      (`SceneComponent.K2_SetRelativeTransform` _overlap (`SceneComponent.GetRelativeTransform` _overlapsource) false false)
      (`BoxComponent.SetBoxExtent` _overlap (`BoxComponent.BoxExtent` _overlapsource) true)
      (`BoxComponent.SetBoxExtent` (`/CustomScenario/Blueprints/BP_CustomButton_PerPlayer.Use` PerPlayerBP) (`BoxComponent.BoxExtent` (`self.UseSource`)) true))
    (:`then_1`
      (set `BlueprintUsableActor.UseHoldBehavior` (`self.UseHoldBehavior`) PerPlayerBP)
      (set `BlueprintUsableActor.UseTime` (`self.UseTime`) PerPlayerBP)
      (set `BlueprintUsableActor.bHasTapAndHoldBehavior` (`self.bHasTapAndHoldBehavior`) PerPlayerBP)
      (set `BlueprintUsableActor.bCanProneWhileUse` (`self.bCanProneWhileUse`) PerPlayerBP)
      (set `BlueprintUsableActor.YawLimitWhileUse` (`self.YawLimitWhileUse`) PerPlayerBP)
      (set `BlueprintUsableActor.UseMessage` (`self.UseMessage`) PerPlayerBP)
      (set `BlueprintUsableActor.UseImage` (`self.UseImage`) PerPlayerBP)
      (set `BlueprintUsableActor.bHasUseTimeout` (`self.bHasUseTimeout`) PerPlayerBP)
      (set `/CustomScenario/Blueprints/BP_CustomButton_PerPlayer.DispatchReplication` (`self.DispatchReplication`) PerPlayerBP)
      (set `/CustomScenario/Blueprints/BP_CustomButton_PerPlayer.createRadial` (`self.createRadialMenu`) PerPlayerBP)
      (set `/CustomScenario/Blueprints/BP_CustomButton_PerPlayer.AntiSpamTimeout` (`self.AntiSpamTimeout`) PerPlayerBP)
      (set `/CustomScenario/Blueprints/BP_CustomButton_PerPlayer.RadialCommands` (`self.RadialCommands`) PerPlayerBP)
      (set `/CustomScenario/Blueprints/BP_CustomButton_PerPlayer.antiSpam` (`self.antiSpam`) PerPlayerBP)
      (`KismetArrayLibrary.Array_Resize` _radial_option_enabled 9)
      ;[0.572 0 0] The binds and dispatchers
      (set `/CustomScenario/Blueprints/BP_CustomButton_PerPlayer.Radial_Option_Enabled` _radial_option_enabled PerPlayerBP))))

(event `RoundCleanup`
  ;[1 0.1342 0.0245] Handle round restarts
  (`self.DestroyAllSpawned`)
  (`KismetArrayLibrary.Array_Clear` (`self.PlayerControllersWithSpawns`)))

(event `FromClient_OnUseCancelled`
  (params (Pawn :type "INSSoldier Object Reference") (SpawnedButton :type "Actor Object Reference"))
  ;[0.572 0 0] The binds and dispatchers
  ;;[1 1 1] onUseCancelled
  (bind _allowed_out (`self.InUseStop` Pawn))
  (if _allowed_out
    (if (`self.DebugOn`)
      (`KismetSystemLibrary.PrintString` "OnUseCancelled"))
    (`self.OnUseCancelledDispatch` Pawn)))

(event `UpdateSpawnedVariables_Event`
  (bind _spawnedbuttons (`self.SpawnedButtons`))
  ;[0.224 0.224 0.224] Spawner vars are replicated so you can dynamically change them. This wont affect already spawned unless you also call this.
  (if (!= (`KismetArrayLibrary.Array_Length` _spawnedbuttons) 0)
    (for _array_element _spawnedbuttons
      (bind _asbp_custom_button_per_player (cast `/CustomScenario/Blueprints/BP_CustomButton_PerPlayer` _array_element))
      (`self.SetSpawnedVariables` _asbp_custom_button_per_player)
      ;;[1 1 1] Update Everyones Buttons
      (if (`self.forceUpdate`)
        (for _array_element_2 (`self.SpawnedButtons`)
          (`self.K2_DestroyActor` _array_element_2))
        (`self.ReEnabled`)))))

(event `FromClient_RecieveRadial`
  (params (Direction :type "ERadialMenuDirection Enum" :default "Radial_North") (Pawn :type "INSSoldier Object Reference") (SpawnedButton :type "Actor Object Reference"))
  ;[0.572 0 0] The binds and dispatchers
  ;;[1 1 1] onRadialSelected
  (bind _allowed_out (`self.InUseStop` Pawn false true))
  (if _allowed_out
    (if (`self.DebugOn`)
      (`KismetSystemLibrary.PrintString` (`|GetEnumeratorNameAsString` Direction)))
    (`self.OnRadialCommandDispatch` Direction Pawn)))

(event `CustomEvent_0`
  (params (Pawn :type "INSSoldier Object Reference") (`Spawned Button` :type "Actor Object Reference"))
  ;[0.572 0 0] The binds and dispatchers
  ;;[1 1 1] onRadialHidden
  (bind _allowed_out (`self.InUseStop` Pawn false true))
  (if _allowed_out
    (if (`self.DebugOn`)
      (`KismetSystemLibrary.PrintString` "OnMenuHide"))
    (`self.OnRadialMenuHiddenDispatch` Pawn)))

(fn `DestroyAllSpawned`
  (bind _spawnedbuttons (`self.SpawnedButtons`))
  (if (!= (`KismetArrayLibrary.Array_Length` _spawnedbuttons) 0)
    (for _array_element _spawnedbuttons
      (`self.K2_DestroyActor` _array_element)))
  (return))

(fn `HideOthersInUse`
  (for _array_element (`self.SpawnedButtons`)
    (if (!= _array_element (`self.SpawnedButton`))
      (`self.K2_DestroyActor` _array_element)))
  (return))

(fn `InUseStart`
  (params (UsingPawn :type "INSSoldier Object Reference") (SpawnedButton :type "Actor Object Reference"))
  (returns (AllowedOut :type Boolean))
  (locals (Allowed :type Boolean))
  (bind _usetime (`self.UseTime`))
  (bind _oneuser (`self.oneUser`))
  (bind _radialtimeout (`self.RadialTimeout`))
  (bind _timer (`self.Timer`))
  (if (or (and _oneuser (!= (`self.UseTime`) 0.0)) (and _oneuser (`self.createRadialMenu`) (`self.RadialEnds_InUse`)))
    (if (== UsingPawn (`self.UsingPawn`))
      (set `self.UsingPawn` UsingPawn :!label _label)
      (set `self.SpawnedButton` SpawnedButton)
      (set `self.buttonInUse` true)
      (if (`KismetSystemLibrary.K2_IsValidTimerHandle` _timer)
        (`KismetSystemLibrary.K2_ClearAndInvalidateTimerHandle` _timer))
      (bind _returnvalue (`KismetSystemLibrary.K2_SetTimer` self "inUseTimeout" (`KismetMathLibrary.SelectFloat` (+ (`KismetMathLibrary.SelectFloat` (+ _radialtimeout 1.0) _radialtimeout (<= _radialtimeout 1.0)) _usetime) (+ _usetime 1.0) (and (`self.createRadialMenu`) (`self.RadialEnds_InUse`)))))
      (set `self.Timer` _returnvalue)
      (if (`self.hide_inUse`)
        _
        (else
          _))
      (set `local.Allowed` true :!label _label_2)
      (elif (`self.buttonInUse`)
        (`KismetSystemLibrary.PrintString` "InUse")
        (set `local.Allowed` false)
        (else
          (goto _label))))
    (else
      (goto _label_2)))
  (return (`local.Allowed`)))

(fn `InUseStop`
  (params (`Using Pawn` :type "INSSoldier Object Reference") (`OnComplete Func` :type Boolean) (`Radial Func` :type Boolean))
  (returns (`Allowed Out` :type Boolean))
  (locals (Allowed :type Boolean))
  (bind _returnvalue (== `Using Pawn` (`self.UsingPawn`)))
  (bind _returnvalue_2 (and (`self.RadialEnds_InUse`) (`self.createRadialMenu`) (`self.oneUser`)))
  (if (or _returnvalue_2 (and (`self.oneUser`) (!= (`self.UseTime`) 0.0)))
    ;[0.002934 0.03942 1] If RadialEnds and OneUser
    (if _returnvalue_2
      (if (not `OnComplete Func`)
        ;[0.04985 1 0.1746] Is the holder
        (if _returnvalue :!label _label
          (set `self.buttonInUse` false)
          (`KismetSystemLibrary.K2_ClearAndInvalidateTimerHandle` (`self.Timer`))
          (set `local.Allowed` true :!label _label_2)
          (else
            (`KismetSystemLibrary.PrintString` "EndNotUser" :!label _label_3)
            (set `local.Allowed` false)))
        (else
          ;[0 0.02768 1] If Radial Ends AND this is onComplete hold. Don't end on use but still send a dispatch if holding user
          (if _returnvalue
            (goto _label_2)
            (else
              (goto _label_3)))))
      (else
        (goto _label)))
    (else
      (goto _label_2)))
  (return (`local.Allowed`)))

(fn `inUseTimeout`
  (set `self.buttonInUse` false)
  (bind _asbp_custom_button_per_player (cast `/CustomScenario/Blueprints/BP_CustomButton_PerPlayer` (`self.SpawnedButton`))
    (:`then`
      (`/CustomScenario/Blueprints/BP_CustomButton_PerPlayer.HideMenuDispatch` _asbp_custom_button_per_player))
    (:`CastFailed`
      _))
  (return))

(fn `OnRep_buttonInUse`
  (if (`self.hide_inUse`)
    (if (`self.buttonInUse`)
      (`self.HideOthersInUse`)
      (else
        (`self.ReEnabled`))))
  (return))

(fn `OnRep_Radial_Option_Enabled`
  (bind _radial_option_enabled (`self.Radial_Option_Enabled`))
  (for _array_element (`self.SpawnedButtons`)
    (bind _asbp_custom_button_per_player (cast `/CustomScenario/Blueprints/BP_CustomButton_PerPlayer` _array_element))
    (`KismetArrayLibrary.Array_Resize` _radial_option_enabled 9)
    (set `/CustomScenario/Blueprints/BP_CustomButton_PerPlayer.Radial_Option_Enabled` _radial_option_enabled _asbp_custom_button_per_player))
  (`/Engine/EditorBlueprintResources/StandardMacros.IsValid` _asbp_custom_button_per_player
    (:`Is Valid`
      ;[1 1 1] Update Everyones Buttons
      (for _array_element_2 (`self.SpawnedButtons`)
        (`self.K2_DestroyActor` _array_element_2))
      (`self.ReEnabled`))
    (:`Is Not Valid`
      _))
  (return))

(fn `OnRep_UseEnabled`
  (bind _enabled (`self.Enabled`))
  ;[0.1198 0.1198 0.1198] Fires when the bool changes due to RepNotify replication
  (if (not (`self.Enabled`))
    (`self.DestroyAllSpawned`))
  (if (`self.EnabledAffectsOverlapEvents`)
    (set `PrimitiveComponent.bGenerateOverlapEvents` _enabled (`self.OverlapSource`)))
  (if _enabled
    (`self.ReEnabled`))
  (return))

(fn `UserConstructionScript`
  (`BillboardComponent.SetSprite` (`self.HintSource`) (`self.UseImage`)))