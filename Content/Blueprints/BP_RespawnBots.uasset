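; Actor that respawns bots of a chosen team standing inside its box volume when a linked objective becomes inactive.
; One second after BeginPlay it caches the INSMultiplayerMode game mode and binds to the objective's active-state delegate.
; On deactivation it gathers overlapping player characters, prints their names, and calls RespawnBot for those on BotTeam with a valid AI controller.
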(event `self.ReceiveBeginPlay`
  (`KismetSystemLibrary.Delay` 1.0)
  (bind _asinsmultiplayer_mode (cast `INSMultiplayerMode` (`GameplayStatics.GetGameMode`)))
  (add `ObjectiveBase.OnObjectiveActiveDelegate` (`|ConvertAsset` (`self.Objective`)) (delegate `onObjectiveActive`)))

(event `onObjectiveActive`
  (params (bNewActiveState :type Boolean) (Objective :type "ObjectiveBase Object Reference"))
  (if (not bNewActiveState)
    (for _array_element (`PrimitiveComponent.GetOverlappingActors` (`self.Box`) "/Game/Game/Actors/Characters/BP_Character_Player.BP_Character_Player_C")
      (bind _asbp_character_player (cast `/Game/Game/Actors/Characters/BP_Character_Player` _array_element))
      (`KismetSystemLibrary.PrintString` (`KismetSystemLibrary.GetObjectName` _asbp_character_player))
      (bind _returnvalue (`INSSoldier.GetAIController` _asbp_character_player))
      (if (and (== (`INSSoldier.TeamId` _asbp_character_player) (`self.BotTeam`)) (`KismetSystemLibrary.IsValid` _returnvalue))
        (`INSGameMode.RespawnBot` (stale `self.ReceiveBeginPlay` _asinsmultiplayer_mode) _returnvalue)))))

(fn `UserConstructionScript`)