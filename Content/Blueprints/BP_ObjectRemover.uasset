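; BP_ObjectRemover suppresses listed level objects on BeginPlay without destroying the actors.
; It resolves actors from RemoveList references and RemoveListString soft paths, then hides their root and descendant primitive components and makes them ignore all collision channels.
; RemoveList also handles Volumes without a primitive root cast by disabling brush collision responses.
; A Removeinstances helper calls RemoveInstance in a forward index loop on any instanced static mesh component.
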(event `self.ReceiveBeginPlay`
  (for _array_element (`self.RemoveList`)
    (bind _output (`|ConvertAsset` _array_element))
    (if (`KismetSystemLibrary.IsValid` _output)
      (`|ExecutionSequence`
        (:`then_0`
          (bind _rootcomponent (`Actor.RootComponent` _output))
          (bind _asprimitive_component (cast `PrimitiveComponent` _rootcomponent)
            (:`then`
              (`SceneComponent.SetVisibility` _asprimitive_component false true)
              (`PrimitiveComponent.SetCollisionResponseToAllChannels` _asprimitive_component "ECR_Ignore")
              (for _array_element_2 (`SceneComponent.GetChildrenComponents` _rootcomponent true)
                (bind _asprimitive_component_2 (cast `PrimitiveComponent` _array_element_2))
                (`PrimitiveComponent.SetCollisionResponseToAllChannels` _asprimitive_component_2 "ECR_Ignore")
                (`SceneComponent.SetVisibility` _asprimitive_component_2 false true)
                (`self.Removeinstances` _asprimitive_component_2)))
            (:`CastFailed`
              (bind _asvolume (cast `Volume` _output))
              (`PrimitiveComponent.SetCollisionResponseToAllChannels` (`Brush.BrushComponent` _asvolume) "ECR_Ignore"))))
        (:`then_1`
          (`self.Removeinstances` _rootcomponent)))))
  (for _array_element_3 (`self.RemoveList_String`)
    (bind _asactor (cast `Actor` (`|ConvertAsset` (`KismetSystemLibrary.Conv_SoftObjPathToSoftObjRef` (`KismetSystemLibrary.MakeSoftObjectPath` _array_element_3)))))
    (bind _rootcomponent_2 (`Actor.RootComponent` _asactor))
    (bind _asprimitive_component_3 (cast `PrimitiveComponent` _rootcomponent_2))
    (`SceneComponent.SetVisibility` _asprimitive_component_3 false true)
    (`PrimitiveComponent.SetCollisionResponseToAllChannels` _asprimitive_component_3 "ECR_Ignore")
    (`self.Removeinstances` _asprimitive_component_3
      (:`Exec`
        (for _array_element_4 (`SceneComponent.GetChildrenComponents` _rootcomponent_2 true)
          (bind _asprimitive_component_4 (cast `PrimitiveComponent` _array_element_4))
          (`PrimitiveComponent.SetCollisionResponseToAllChannels` _asprimitive_component_4 "ECR_Ignore")
          (`SceneComponent.SetVisibility` _asprimitive_component_4 false true)
          (`self.Removeinstances` _asprimitive_component_4))))))

(fn `UserConstructionScript`)