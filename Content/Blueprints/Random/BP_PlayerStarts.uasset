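; BP_PlayerStarts is a placeable actor that snaps its child components, presumably player spawn points, onto the ground.
; Construct traces down from each child, caches the hit raised by a fixed offset (or the original position on a miss), moves the children there, then calls FindSpawnsDispatch.
; The construction script clears the cache and rebuilds when the actor transform changes.
; FindSpawns2 reruns Construct, which only reapplies cached locations when they exist.
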(event `Construct`
  (bind _worldlocation (`self.WorldLocation`))
  (bind _children (`SceneComponent.GetChildrenComponents` (`self.RootComponent`) false))
  (if (`KismetArrayLibrary.Array_IsValidIndex` (`self.WorldLocation`)) :!label _label
    (for (_array_element _array_index) _children :!label _label_2
      (`SceneComponent.K2_SetWorldLocation` _array_element (`|GetArrayItem` (`self.WorldLocation`) _array_index) false false))
    (else
      (`KismetArrayLibrary.Array_Clear` (`self.WorldLocation`))
      (for _array_element_2 _children
        (bind _returnvalue (`SceneComponent.K2_GetComponentLocation` _array_element_2))
        (bind (_outhit _returnvalue_2) (`KismetSystemLibrary.LineTraceSingle` :`Start` _returnvalue :`End` (+ _returnvalue (0.0 0.0 -10000.0)) :`TraceChannel` "TraceTypeQuery5" :`DrawTime` 0.2))
        (if _returnvalue_2
          (`KismetArrayLibrary.Array_Add` _worldlocation (+ (`.Location` (`GameplayStatics.BreakHitResult` _outhit)) (0.0 0.0 90.0)))
          (else
            (`KismetArrayLibrary.Array_Add` _worldlocation _returnvalue))))
      (`|ExecutionSequence`
        (:`then_0`
          (goto _label_2))
        (:`then_1`
          (`self.FindSpawnsDispatch`))))))

(event `FindSpawns2`
  (goto _label))

(fn `UserConstructionScript`
  (bind _returnvalue (`self.GetTransform` self))
  (if (not (`KismetMathLibrary.NearlyEqual_TransformTransform` (`self.LastConstruct`) _returnvalue))
    (set `self.LastConstruct` _returnvalue)
    (`KismetArrayLibrary.Array_Clear` (`self.WorldLocation`))
    (`self.Construct`)))