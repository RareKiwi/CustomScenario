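; Placeable objective point for randomized multiplayer layouts, bound by index to one of the scenario's objectives.
; It either spawns a weapon cache mirroring that objective's active state, or copies its collision shapes onto the territory objective.
; Cache destruction briefly switches the objective's type to hand it to the attackers.
; Given a layout, it relocates attacker spawn zones with their player starts, and counter-attack zones, choosing spawns by distance to neighboring points.
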(event `CacheObjectiveSync`
  (params (bNewActiveState :type Boolean) (Objective :type "ObjectiveBase Object Reference"))
  (bind _cache (`self.Cache`))
  (if (`KismetSystemLibrary.IsValid` _cache)
    (`ObjectiveBase.SetObjectiveActive` _cache bNewActiveState)))

(event `RoundCleanup`
  (bind _cache (`self.Cache`))
  (bind _objective (`self.Objective`))
  (bind _cache_2 (`self.Cache`))
  (bind _returnvalue (`ObjectiveBase.GetActive` _objective))
  (if (`KismetSystemLibrary.IsValid` _cache)
    (`self.K2_DestroyActor` _cache))
  (if (`self.isCache`)
    (bind _returnvalue_2 (`|SpawnActorFromClass` "/Game/Game/Actors/Objectives/Obj_WeaponCache_Ins.Obj_WeaponCache_Ins_C" (`KismetMathLibrary.MakeTransform` (- (`self.K2_GetActorLocation`) (0.0 0.0 150.0)) (`self.K2_GetActorRotation`)) "AlwaysSpawn" "OverrideRootScale" null null))
    (set `self.Cache` _returnvalue_2)
    (`KismetSystemLibrary.Delay` 0.1)
    (add `ObjectiveDestructible.OnDestructibleObjectiveStateChangedDelegate` _returnvalue_2 (`|CreateDelegate` :!event `CustomEvent_0`))
    (clear `ObjectiveBase.OnObjectiveActiveDelegate` _objective :!label _label)
    (`KismetSystemLibrary.Delay` 0.1)
    (add `ObjectiveBase.OnObjectiveActiveDelegate` _objective (delegate `CustomEvent`))
    (`ObjectiveBase.SetObjectiveActive` _cache_2 _returnvalue)
    (`ObjectiveBase.SetLockedForTeam` _cache_2 (`self.AttackingTeam`) (not _returnvalue))))

(event `CleanupObjectives`
  (bind _cache (`self.Cache`))
  (if (`KismetSystemLibrary.IsValid` _cache)
    (`self.K2_DestroyActor` _cache))
  (`self.RemoveCollisions`))

(event `CustomEvent`
  (params (bNewActiveState :type Boolean) (Objective :type "ObjectiveBase Object Reference"))
  (bind _cache (`self.Cache`))
  (`ObjectiveBase.SetObjectiveActive` _cache bNewActiveState)
  (`ObjectiveBase.SetLockedForTeam` _cache (`self.AttackingTeam`) (not bNewActiveState)))

(event `SetupObjectives`
  (bind (_attackingteam _defendingteam _objective) (`self.FuncGetObjective` (`self.ObjectiveIndex`)))
  (set `self.AttackingTeam` _attackingteam)
  (set `self.DefendingTeam` _defendingteam)
  (set `self.Objective` _objective)
  (if (`self.isCache`)
    (`self.DisableTerritory`)
    (`KismetSystemLibrary.PrintString` (`KismetStringLibrary.Concat_StrStr` "Cache spawned at " (`KismetStringLibrary.Conv_ByteToString` (`self.ObjectiveIndex`))))
    (bind _returnvalue (`|SpawnActorFromClass` "/Game/Game/Actors/Objectives/Obj_WeaponCache_Ins.Obj_WeaponCache_Ins_C" (`KismetMathLibrary.MakeTransform` (- (`self.K2_GetActorLocation`) (0.0 0.0 150.0)) (`self.K2_GetActorRotation`)) "AlwaysSpawn" "OverrideRootScale" null null))
    (set `self.Cache` _returnvalue)
    (`KismetSystemLibrary.Delay` 0.1)
    (add `ObjectiveDestructible.OnDestructibleObjectiveStateChangedDelegate` _returnvalue (`|CreateDelegate` :!event `CustomEvent_0`))
    (goto _label)
    (else
      (`self.EnableTerritory`)
      (`self.MakeCollision`))))

(event `self.ReceiveBeginPlay`
  (if (`KismetSystemLibrary.IsServer`)
    (for _array_element (`SceneComponent.GetChildrenComponents` (`self.Box`) true)
      (if (`KismetArrayLibrary.Array_Contains` (`|MakeArray` "/Script/Engine.BoxComponent" "/Script/Engine.SphereComponent" "/Script/Engine.CapsuleComponent" :!type "SceneComponent Class Reference") (`GameplayStatics.GetObjectClass` _array_element))
        (bind _asprimitive_component (cast `PrimitiveComponent` _array_element))
        (`KismetArrayLibrary.Array_Add` (`self.Components`) _asprimitive_component)))))

(event `CustomEvent_0`
  (params (Objective :type "ObjectiveDestructible Object Reference") (NewState :type "EDestructibleObjectiveState Enum" :default "Normal"))
  (bind _objective (`self.Objective`))
  (if (`|EnumEquality` NewState "Destroyed")
    (`/Engine/EditorBlueprintResources/StandardMacros.DoOnce` false :!label _label_2
      (:`Completed`
        (`|ExecutionSequence`
          (:`then_0`
            (set `ObjectiveBase.ObjectiveType` "Object" _objective)
            (`KismetSystemLibrary.Delay` 0.1)
            (`ObjectiveBase.SetOwningTeam` _objective (`self.AttackingTeam`))
            (`KismetSystemLibrary.Delay` 0.1)
            (set `ObjectiveBase.ObjectiveType` "Territory" _objective))
          (:`then_1`
            (`KismetSystemLibrary.Delay` 0.2)
            (goto _label_2 :!via `Reset`)))))))

(fn `DisableTerritory`
  (bind _asobjective_capturable (cast `ObjectiveCapturable` (`self.Objective`))
    (:`then`
      (bind _asprimitive_component (cast `PrimitiveComponent` (`Actor.RootComponent` _asobjective_capturable))
        (:`then`
          (`PrimitiveComponent.SetCollisionProfileName` _asprimitive_component "NoCollision" true)
          (return))
        (:`CastFailed`
          (return))))
    (:`CastFailed`
      (return))))

(fn `EnableTerritory`
  (bind _asobjective_capturable (cast `ObjectiveCapturable` (`self.Objective`))
    (:`then`
      (bind _asprimitive_component (cast `PrimitiveComponent` (`Actor.RootComponent` _asobjective_capturable))
        (:`then`
          (`PrimitiveComponent.SetCollisionProfileName` _asprimitive_component "Trigger" true)
          (return))
        (:`CastFailed`
          (return))))
    (:`CastFailed`
      (return))))

(fn `FuncGetObjective`
  (params (ID :type Byte))
  (returns (AttackingTeam :type Byte) (DefendingTeam :type Byte) (Objective :type "ObjectiveBase Object Reference"))
  (bind _asinsmultiplayer_mode (cast `INSMultiplayerMode` (`GameplayStatics.GetGameMode`))
    (:`then`
      (return (`INSGameMode.GetAttackingTeam` _asinsmultiplayer_mode) (`INSGameMode.GetDefendingTeam` _asinsmultiplayer_mode) (`|ConvertAsset` (`.Objective` (break `ObjectiveInfo` (`|GetArrayItem` (`ScenarioBase.Objectives` (`INSMultiplayerMode.MultiplayerScenario` _asinsmultiplayer_mode)) (`KismetMathLibrary.Conv_ByteToInt` ID)))))))
    (:`CastFailed`
      (`KismetSystemLibrary.PrintString` "Hello")
      (return 0 0 null))))

(fn `GetSpawnZone`
  (params (index :type Byte))
  (returns (Starts :type "Array of INSPlayerStart Object Reference") (SpawnZone :type "SpawnZone Object Reference") (Valid :type Boolean))
  (locals (NewLocalVar_0 :type "Array of INSPlayerStart Object Reference") (NewLocalVar_1 :type "SpawnZone Object Reference") (NewLocalVar_2 :type Boolean :default false))
  (bind _asinsmultiplayer_mode (cast `INSMultiplayerMode` (`GameplayStatics.GetGameMode`))
    (:`then`
      (for _array_element (`.SpawnZones` (break `ObjectiveInfo` (`|GetArrayItem` (`ScenarioBase.Objectives` (`INSMultiplayerMode.MultiplayerScenario` _asinsmultiplayer_mode)) (`KismetMathLibrary.Conv_ByteToInt` index))))
        (bind _output (`|ConvertAsset` _array_element))
        (if (== (`INSGameMode.GetAttackingTeam` _asinsmultiplayer_mode) (`SpawnZone.TeamId` _output))
          (set `local.NewLocalVar_1` _output)
          (set `local.NewLocalVar_0` (`SpawnZone.PlayerStarts` _output))
          (set `local.NewLocalVar_2` true)
          (break)))
      (return (`local.NewLocalVar_0`) (`local.NewLocalVar_1`) (`local.NewLocalVar_2`)))
    (:`CastFailed`
      (return _ null false))))

(fn `GetSpawnZoneCA`
  (params (index :type Byte))
  (returns (SpawnZone :type "SpawnZone Object Reference") (Valid :type Boolean))
  (locals (NewLocalVar_1 :type "SpawnZone Object Reference") (NewLocalVar_2 :type Boolean :default false))
  (bind _asinsmultiplayer_mode (cast `INSMultiplayerMode` (`GameplayStatics.GetGameMode`))
    (:`then`
      (for _array_element (`.SpawnZones` (break `ObjectiveInfo` (`|GetArrayItem` (`ScenarioBase.Objectives` (`INSMultiplayerMode.MultiplayerScenario` _asinsmultiplayer_mode)) (`KismetMathLibrary.Conv_ByteToInt` index))))
        (bind _output (`|ConvertAsset` _array_element))
        (if (!= (`INSGameMode.GetAttackingTeam` _asinsmultiplayer_mode) (`SpawnZone.TeamId` _output))
          (set `local.NewLocalVar_1` _output)
          (set `local.NewLocalVar_2` true)
          (break)))
      (return (`local.NewLocalVar_1`) (`local.NewLocalVar_2`)))
    (:`CastFailed`
      (return null false))))

(fn `MakeCollision`
  (returns (Valid :type Boolean))
  (bind _objective (`self.Objective`))
  (bind _spawnedcomponents (`self.SpawnedComponents`))
  (bind _returnvalue (`KismetSystemLibrary.IsValid` _objective))
  (if (`KismetSystemLibrary.IsServer`)
    (if _returnvalue
      (for _array_element (`self.Components`)
        (bind _asbox_collision (cast `BoxComponent` _array_element)
          (:`then`
            (bind _returnvalue_2 (`SceneComponent.GetRelativeTransform` _array_element))
            (bind _returnvalue_3 (`AddComponent|NODE_AddBoxComponent-0` :`self` _objective :`RelativeTransform` _returnvalue_2))
            (`BoxComponent.SetBoxExtent` _returnvalue_3 (`BoxComponent.GetUnscaledBoxExtent` _asbox_collision) true)
            (`KismetArrayLibrary.Array_Add` _spawnedcomponents _returnvalue_3))
          (:`CastFailed`
            (bind _ascapsule_collision (cast `CapsuleComponent` _array_element)
              (:`then`
                (bind _returnvalue_4 (`AddComponent|NODE_AddCapsuleComponent-0` :`self` _objective :`RelativeTransform` _returnvalue_2))
                (`CapsuleComponent.SetCapsuleSize` _returnvalue_4 (`CapsuleComponent.CapsuleRadius` _ascapsule_collision) (`CapsuleComponent.CapsuleHalfHeight` _ascapsule_collision) true)
                (`KismetArrayLibrary.Array_Add` _spawnedcomponents _returnvalue_4))
              (:`CastFailed`
                (bind _assphere_collision (cast `SphereComponent` _array_element))
                (bind _returnvalue_5 (`AddComponent|NODE_AddSphereComponent-0` :`self` _objective :`RelativeTransform` _returnvalue_2))
                (`SphereComponent.SetSphereRadius` _returnvalue_5 (`SphereComponent.GetUnscaledSphereRadius` _assphere_collision) true)
                (`KismetArrayLibrary.Array_Add` _spawnedcomponents _returnvalue_5)))))))
    (return _returnvalue)))

(fn `MovePlayerStarts`
  (params (BP_Start :type "Actor Object Reference") (Starts :type "Array of INSPlayerStart Object Reference") (TargetToLookAt :type "Vector Structure"))
  (bind _starts (`local.Starts`))
  (bind _capsulespawns (`self.CapsuleSpawns`))
  (set `self.CapsuleSpawns` (`SceneComponent.GetChildrenComponents` (`Actor.RootComponent` (`local.BP_Start`)) false))
  (for _array_element _capsulespawns
    (cast `CapsuleComponent` _array_element
      (:`CastFailed`
        (`KismetArrayLibrary.Array_RemoveItem` _capsulespawns _array_element))))
  (for (_array_element_2 _array_index) _capsulespawns
    (if (< _array_index (`KismetArrayLibrary.Array_Length` _starts))
      (bind _output (`|GetArrayItem` _starts _array_index))
      (`SceneComponent.SetMobility` (`Actor.RootComponent` _output) "Movable")
      (bind _returnvalue (`SceneComponent.K2_GetComponentLocation` _array_element_2))
      (`self.K2_SetActorLocation` _output _returnvalue false false)
      (`self.K2_SetActorRotation` _output (`KismetMathLibrary.Conv_VectorToRotator` (`KismetMathLibrary.Vector_Normal2D` (- (`local.TargetToLookAt`) _returnvalue))) false)))
  (return))

(fn `OnRep_Objective`
  (`KismetSystemLibrary.PrintString` "Objectiveset")
  (`KismetSystemLibrary.PrintString` (`KismetStringLibrary.Concat_StrStr` "Reped " (`KismetStringLibrary.Conv_ByteToString` (`self.ObjectiveIndex`))))
  (return))

(fn `RemoveCollisions`
  (returns (Valid :type Boolean))
  (bind _returnvalue (`KismetSystemLibrary.IsValid` (`self.Objective`)))
  (if (`KismetSystemLibrary.IsServer`)
    (if _returnvalue
      (for _array_element (`self.SpawnedComponents`)
        (`PrimitiveComponent.SetCollisionEnabled` _array_element "NoCollision")))
    (return _returnvalue)))

(fn `SetupCounterAttackSpawns`
  (params (Layout :type "Array of /Game/Blueprints/Random/BP_ObjectiveRandom Object Reference"))
  (locals (Distance :type "Float (double-precision)" :default 10000000.0) (BPPlayerStart :type "/CustomScenario/Blueprints/Random/BP_PlayerStarts Object Reference"))
  (if (!= (`KismetArrayLibrary.Array_LastIndex` (`local.Layout`)) (`KismetMathLibrary.Conv_ByteToInt` (`self.ObjectiveIndex`)))
    (for _array_element (`self.PlayerSpawns`)
      (bind _output (`|ConvertAsset` _array_element))
      (if (`KismetSystemLibrary.IsValid` _output)
        (bind _returnvalue (`self.GetDistanceTo` _output (`|GetArrayItem` (`local.Layout`) (`KismetMathLibrary.Conv_ByteToInt` (+ (`self.ObjectiveIndex`) 1)))))
        (if (< _returnvalue (`local.Distance`))
          (set `local.Distance` _returnvalue)
          (set `local.BPPlayerStart` _output))))
    (if (`KismetSystemLibrary.IsValid` (`local.BPPlayerStart`))
      (bind (_spawnzone _valid) (`self.GetSpawnZoneCA` (`self.ObjectiveIndex`)))
      (if _valid
        (set `self.CounterAttackSpawnZone` _spawnzone)
        (`SceneComponent.SetMobility` (`Brush.BrushComponent` _spawnzone) "Movable")
        (`self.K2_SetActorLocation` _spawnzone (`self.K2_GetActorLocation` (`local.BPPlayerStart`)) false false)
        (return)
        (else
          (return)))
      (else
        (return)))
    (else
      (set `local.Distance` 0.0)
      (for _array_element_2 (`self.PlayerSpawns`)
        (bind _output_2 (`|ConvertAsset` _array_element_2))
        (bind _returnvalue_2 (`self.GetDistanceTo` _output_2 (`|GetArrayItem` (`local.Layout`) (`KismetMathLibrary.Conv_ByteToInt` (- (`self.ObjectiveIndex`) 1)))))
        (if (> _returnvalue_2 (`local.Distance`))
          (set `local.Distance` _returnvalue_2)
          (set `local.BPPlayerStart` _output_2)))
      (if (`KismetSystemLibrary.IsValid` (`local.BPPlayerStart`))
        (bind (_spawnzone_2 _valid_2) (`self.GetSpawnZoneCA` (`self.ObjectiveIndex`)))
        (if _valid_2
          (set `self.CounterAttackSpawnZone` _spawnzone_2)
          (`SceneComponent.SetMobility` (`Brush.BrushComponent` _spawnzone_2) "Movable")
          (`self.K2_SetActorLocation` _spawnzone_2 (`self.K2_GetActorLocation` (`local.BPPlayerStart`)) false false)
          (return)
          (else
            (return)))
        (else
          (return))))))

(fn `SetupPlayerSpawns1`
  (params (Layout :type "Array of /Game/Blueprints/Random/BP_ObjectiveRandom Object Reference"))
  (returns (CrateTransform :type "Transform Structure") (PlayerSpawnZones :type "Transform Structure") (CASpawnZones :type "Transform Structure") (SpawnZone :type "SpawnZone Object Reference") (Objective :type "ObjectiveBase Object Reference") (SpawnZoneName :type String))
  (bind _pickedspawn (`self.PickedSpawn`))
  (bind _objective (`self.Objective`))
  (bind _objectiveindex (`self.ObjectiveIndex`))
  (bind _objective_2 (`self.Objective`))
  (bind _objective_3 (`self.Objective`))
  (bind _output (`|ConvertAsset` (`|GetArrayItem` (`self.PlayerSpawnsBeginRound`))))
  (bind _output_2 (`|ConvertAsset` (`/CustomScenario/Blueprints/Random/BP_PlayerStarts.Crate` _pickedspawn)))
  (bind _output_3 (`|ConvertAsset` (`/CustomScenario/Blueprints/Random/BP_PlayerStarts.Crate` _output)))
  (if (and (`self.Start Objective`) (== (`self.ObjectiveIndex`) 0))
    (bind (_starts _spawnzone _valid) (`self.GetSpawnZone` 0))
    (if _valid
      (if (`KismetSystemLibrary.IsValid` _output)
        (`SceneComponent.SetMobility` (`Brush.BrushComponent` _spawnzone) "Movable")
        (`self.K2_SetActorLocation` _spawnzone (`self.K2_GetActorLocation` _output) false false)
        (`self.MovePlayerStarts` _output _starts (`self.K2_GetActorLocation` (`self.Objective`)))
        (if (`KismetSystemLibrary.IsValid` _output_3)
          (bind _returnvalue (`self.GetTransform` _spawnzone))
          (bind _returnvalue_2 (`KismetSystemLibrary.GetObjectName` _spawnzone))
          (return (`self.GetTransform` _output_3) _returnvalue (struct) _spawnzone _objective_3 _returnvalue_2)
          (else
            (return (struct) _returnvalue (struct) _spawnzone _objective_3 _returnvalue_2)))
        (else
          (return (struct) (struct) (struct) null _objective_2 "")))
      (else
        (return (struct) (struct) (struct) null _objective_2 "")))
    (elif (!= _objectiveindex 0)
      (bind (_starts_2 _spawnzone_2 _valid_2) (`self.GetSpawnZone` _objectiveindex))
      (if _valid_2
        (set `self.BiggestDistance` 0.0)
        (set `self.PickedSpawn` null)
        (for _array_element (`/Game/Blueprints/Random/BP_ObjectiveRandom.PlayerSpawns` (`|GetArrayItem` Layout (`KismetMathLibrary.Conv_ByteToInt` (- _objectiveindex 1))))
          (bind _output_4 (`|ConvertAsset` _array_element))
          (if (`KismetSystemLibrary.IsValid` _output_4)
            (bind _returnvalue_3 (`self.GetDistanceTo` _output_4 self))
            (if (> _returnvalue_3 (`self.BiggestDistance`))
              (set `self.BiggestDistance` _returnvalue_3)
              (set `self.PickedSpawn` _output_4))))
        (if (`KismetSystemLibrary.IsValid` (`self.PickedSpawn`))
          (`SceneComponent.SetMobility` (`Brush.BrushComponent` _spawnzone_2) "Movable")
          (`self.K2_SetActorLocation` _spawnzone_2 (`self.K2_GetActorLocation` _pickedspawn) false false)
          (bind _asinsmultiplayer_mode (cast `INSMultiplayerMode` (`GameplayStatics.GetGameMode`))
            (:`then`
              (bind _output_objective (break `ObjectiveInfo` (`|GetArrayItem` (`ScenarioBase.Objectives` (`INSMultiplayerMode.MultiplayerScenario` _asinsmultiplayer_mode)) (`KismetMathLibrary.Conv_ByteToInt` (- (`self.ObjectiveIndex`) 1)))))
              (`self.MovePlayerStarts` _pickedspawn _starts_2 (* (+ (`self.K2_GetActorLocation` (`|ConvertAsset` _output_objective)) (`self.K2_GetActorLocation` (`self.Objective`))) 0.5))
              (if (`KismetSystemLibrary.IsValid` _output_2)
                (bind _returnvalue_4 (`self.GetTransform` _spawnzone_2))
                (bind _returnvalue_5 (`KismetSystemLibrary.GetObjectName` _spawnzone_2))
                (return (`self.GetTransform` _output_2) _returnvalue_4 (struct) _spawnzone_2 _objective _returnvalue_5)
                (else
                  (return (struct) _returnvalue_4 (struct) _spawnzone_2 _objective _returnvalue_5))))
            (:`CastFailed`
              (return (struct) (struct) (struct) null (`self.Objective`) "")))
          (else
            (return (struct) (struct) (struct) null (`self.Objective`) "")))
        (else
          (return (struct) (struct) (struct) null (`self.Objective`) "")))
      (else
        (return (struct) (struct) (struct) null null "")))))

(fn `UserConstructionScript`
  (`KismetArrayLibrary.Array_Clear` (`self.Arrows`))
  (`|ExecutionSequence`
    (:`then_1`
      (bind _returnvalue (`AddComponent|NODE_AddStaticMeshComponent-2`))
      (if (`|EnumEquality` (`self.ObjectiveType`) "NewEnumerator2")
        (`StaticMeshComponent.SetStaticMesh` _returnvalue "/Engine/EngineMeshes/Cube.Cube"))
      (`SceneComponent.K2_SetWorldLocation` _returnvalue (+ (`self.K2_GetActorLocation` self) (0.0 0.0 3000.0)) false false)
      (if (not (`self.Start Objective`))
        (`PrimitiveComponent.SetMaterial` _returnvalue 0 "/CustomScenario/Environment/Materials/MI_Blue.MI_Blue")
        (`PrimitiveComponent.SetMaterial` _returnvalue 1 "/CustomScenario/Environment/Materials/MI_Blue.MI_Blue")))
    (:`then_2`
      (if (> (`self.ObjectiveType`) 0)
        (`AddComponent|NODE_AddStaticMeshComponent-3` :`RelativeTransform` (`KismetMathLibrary.MakeTransform` (0.0 0.0 -150.0)))))))