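; Test actor that visualizes 2D Sobol quasi-random point distribution by scattering scaled static mesh components inside a box.
; Construct, run from the construction script, adds one mesh per index at a seeded RandomSobolCell2D position mapped onto the stored bounds at a single height.
; SobolGetBounds caches the Box extent and actor-relative origin separately.
; RandomizeSeed picks a new seed and reruns Construct without removing existing meshes.
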(event `Construct`
  (bind _spheresize (`self.SphereSize`))
  (bind _bounds (`self.Bounds`))
  (for _index (range (+ (`self.MaxIndex`) 1))
    (bind (_returnvalue_x _returnvalue_y) (`KismetMathLibrary.BreakVector2D` (`ImportanceSamplingLibrary.RandomSobolCell2D` _index (`self.NumCells`) (0.0 0.0) (`KismetMathLibrary.ClampAxes2D` (`self.Seed`) 0.0 1.0))))
    (`AddComponent|NODE_AddStaticMeshComponent-4` :`RelativeTransform` (`KismetMathLibrary.MakeTransform` (+ (* (`KismetMathLibrary.MakeVector` _returnvalue_x _returnvalue_y) _bounds (2.0 2.0 2.0)) (- (`self.Origin`) _bounds)) (struct) (`KismetMathLibrary.MakeVector` _spheresize _spheresize _spheresize)))))

(event `SobolGetBounds`
  (bind (_origin _boxextent) (`KismetSystemLibrary.GetComponentBounds` (`self.Box`)))
  (set `self.Bounds` _boxextent)
  (set `self.Origin` (- _origin (`self.K2_GetActorLocation`))))

(event `Randomize Seed`
  (set `self.Seed` (`KismetMathLibrary.MakeVector2D` (`KismetMathLibrary.RandomFloat`) (`KismetMathLibrary.RandomFloat`)))
  (`self.Construct`))

(fn `UserConstructionScript`
  (`self.Construct`))