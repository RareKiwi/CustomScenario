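; BP_RemoveClasses is a Blueprint that removes actors of configured classes from specified worlds when play begins.
; On BeginPlay it converts the Worlds entries to path strings, then synchronously loads each ActorClass entry and gathers all actors of that class.
; An actor is destroyed when its path name starts with one of those world paths, ignoring case, so matching actors outside the listed worlds remain.
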(event `self.ReceiveBeginPlay`
  (for _array_element (`self.Worlds`)
    (`KismetArrayLibrary.Array_Add` (`self.Paths`) (`KismetSystemLibrary.Conv_SoftObjectReferenceToString` _array_element)))
  (for _array_element_2 (`self.ActorClass`)
    (bind _returnvalue (`KismetSystemLibrary.LoadClassAsset_Blocking` _array_element_2))
    (if (`KismetSystemLibrary.IsValidClass` _returnvalue)
      (bind _asactor (castclass `Actor` _returnvalue))
      (bind _outactors (`GameplayStatics.GetAllActorsOfClass` _asactor))
      (for _array_element_3 _outactors
        (for _array_element_4 (`self.Paths`)
          (if (`KismetStringLibrary.StartsWith` (`KismetSystemLibrary.GetPathName` _array_element_3) _array_element_4)
            (`|ExecutionSequence`
              (:`then_0`
                (`self.K2_DestroyActor` _array_element_3))
              (:`then_1`
                (break)))))))))

(fn `UserConstructionScript`)