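; BP_AI_FireAvoider is a placeable actor that keeps a fake fire projectile at its location, apparently so AI avoids that spot.
; On the server, Tick caches the INS multiplayer game mode once and waits for the RoundActive match state.
; It then spawns BP_Projectile_FakeFire, stores the reference, and spawns another whenever that projectile becomes invalid.
; Clients disable their tick.
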(event `self.ReceiveTick`
  (params (DeltaSeconds :type "Float (single-precision)"))
  (bind _returnvalue (`GameplayStatics.GetGameMode`))
  (`/Engine/EditorBlueprintResources/ActorMacros.Switch Has Authority`
    (:`Authority`
      (if (`KismetSystemLibrary.IsValid` (`self.NewVar_0`))
        _
        (elif (`KismetSystemLibrary.IsValid` _returnvalue)
          (`|ExecutionSequence`
            (:`then_0`
              (`/Engine/EditorBlueprintResources/StandardMacros.DoOnce` false
                (:`Completed`
                  (bind _asinsmultiplayer_mode (cast `INSMultiplayerMode` _returnvalue)))))
            (:`then_1`
              (if (== (`GameMode.GetMatchState` _asinsmultiplayer_mode) "RoundActive")
                (bind _returnvalue_2 (`WeaponStatics.SpawnSingleProjectile` "/CustomScenario/Blueprints/PlayerBlockers/BP_Projectile_FakeFire.BP_Projectile_FakeFire_C" null (`self.K2_GetActorLocation`) (0.0 0.0 0.0) null))
                (set `self.NewVar_0` _returnvalue_2)))))))
    (:`Remote`
      (`self.SetActorTickEnabled` false))))

(fn `UserConstructionScript`)