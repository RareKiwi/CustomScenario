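; BP_AITester is a development-only tool that spawns test AI soldiers and makes them chase the first player to exercise navigation.
; On the server, outside distribution builds, it respawns its pawns whenever a round becomes active.
; A looping timer orders each soldier toward the player, choosing near or far move type from current path length.
; It tags action components "Ignore" and flags spawned player-character pawns as ignored by AI.
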(event `self.ReceiveBeginPlay`
  (if (not (`KismetSystemLibrary.IsPackagedForDistribution`))
    (`/Engine/EditorBlueprintResources/ActorMacros.Switch Has Authority`
      (:`Authority`
        (`KismetSystemLibrary.K2_SetTimerDelegate` (delegate `CustomEvent_0`) (`self.Timer`) true)
        (`KismetSystemLibrary.Delay` 1.0)
        (bind _asinsmultiplayer_mode (cast `INSMultiplayerMode` (`GameplayStatics.GetGameMode`)))
        (add `INSMultiplayerMode.OnRoundActiveDelegate` _asinsmultiplayer_mode (delegate `OnRoundActiveDelegate_Event_0`))))))

(event `OnRoundActiveDelegate_Event_0`
  (`self.CleanupSpawnedPawns`)
  (`self.SpawnPawns`)
  (`KismetSystemLibrary.Delay` 0.1)
  (bind _asbp_character_player (cast `/Game/Game/Actors/Characters/BP_Character_Player` (`|GetArrayItem` (`self.GetSpawnedPawns`))))
  (set `INSSoldier.bIgnoredByAI` true _asbp_character_player))

(event `CustomEvent_0`
  (bind _returnvalue (`GameplayStatics.GetPlayerController` 0))
  (bind _returnvalue_2 (`Controller.K2_GetPawn` _returnvalue))
  (for _array_element (`self.GetSpawnedPawns`)
    (if (`KismetSystemLibrary.IsValid` _returnvalue)
      (if (`KismetSystemLibrary.IsValid` _returnvalue_2)
        (bind _asinsaisoldier_controller (cast `INSAISoldierController` (`AIBlueprintHelperLibrary.GetAIController` _array_element)))
        (`KismetArrayLibrary.Array_AddUnique` (`ActorComponent.ComponentTags` (`AIController.ActionsComp` _asinsaisoldier_controller)) "Ignore")
        (`INSAISoldierController.ToggleMovement` _asinsaisoldier_controller true)
        (`INSAISoldierController.MoveToLocationSafe` _asinsaisoldier_controller (`self.K2_GetActorLocation` _returnvalue_2) "Testing" (select `bool` (> (`NavigationPath.GetPathLength` (`AIBlueprintHelperLibrary.GetCurrentPath` _asinsaisoldier_controller)) (`self.FarDistance`)) :`false` (`self.MoveTypeNear`) :`true` (`self.MoveTypeFar`)) "Stand" "Normal" false (`self.AcceptRadius`) (`self.AllowPartial`))
        (bind _asbp_character_player (cast `/Game/Game/Actors/Characters/BP_Character_Player` _array_element))
        (set `INSSoldier.bIgnoredByAI` true _asbp_character_player)))))

(fn `UserConstructionScript`)