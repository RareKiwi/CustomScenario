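; BP_BlockingVolume is a player-blocker volume whose box collision can be switched on and off.
; The construction script applies the configurable collision profile, and BeginPlay disables collision if the volume starts disabled.
; The Enabled RepNotify toggles collision and broadcasts the new state through an event dispatcher.
; An optional Parent reference lets the volume mirror that parent's Enabled changes through its dispatcher, so toggles can cascade.
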(event `self.ReceiveBeginPlay`
  (bind _output (`|ConvertAsset` (`self.Parent`)))
  (if (not (`self.Enabled`))
    (`PrimitiveComponent.SetCollisionEnabled` (`self.Box`) "NoCollision"))
  (if (`KismetSystemLibrary.IsValid` _output)
    (add `self.DispatchEnabled` _output (delegate `ParentEnabled`))))

(event `ParentEnabled` :!signature `self.DispatchEnabled`
  (params (Enabled :type Boolean))
  (set `self.Enabled` Enabled))

(event `DispatchEnabled_Event`
  (params (Enabled :type Boolean)))

(fn `OnRep_Enabled`
  (bind _enabled (`self.Enabled`))
  (`PrimitiveComponent.SetCollisionEnabled` (`self.Box`) (select `bool` _enabled :`false` "NoCollision" :`true` "QueryAndPhysics" :!type "ECollisionEnabled Enum"))
  (`self.DispatchEnabled` _enabled)
  (return))

(fn `UserConstructionScript`
  (`PrimitiveComponent.SetCollisionProfileName` (`self.Box`) (`self.Profile`) true))