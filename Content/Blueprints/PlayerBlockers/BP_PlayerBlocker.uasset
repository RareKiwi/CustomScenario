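; Barrier that blocks player-controlled characters while letting AI characters pass, with a configurable mesh.
; An enlarged box around the blocking volume detects AI, switches Pawn response to Overlap and enables Tick until no bots remain.
; Meanwhile Tick shoves overlapping players out along the chosen local axis and can make AI jump.
; Replicated Enabled state toggles collision and visibility, can follow a parent's dispatcher, and is rebroadcast on change.
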(event `Update`
  (`self.Func_SetAIBox`))

(event `self.BoxCollision.OnComponentBeginOverlap`
  (params (OverlappedComponent :type "PrimitiveComponent Object Reference") (OtherActor :type "Actor Object Reference") (OtherComp :type "PrimitiveComponent Object Reference") (OtherBodyIndex :type Integer) (bFromSweep :type Boolean) (SweepResult :type "HitResult Structure (by ref)")))

(event `self.BoxAI.OnComponentBeginOverlap`
  (params (OverlappedComponent :type "PrimitiveComponent Object Reference") (OtherActor :type "Actor Object Reference") (OtherComp :type "PrimitiveComponent Object Reference") (OtherBodyIndex :type Integer) (bFromSweep :type Boolean) (SweepResult :type "HitResult Structure (by ref)"))
  (if (`self.Enabled`)
    (bind _asbp_character_player (cast `/Game/Game/Actors/Characters/BP_Character_Player` OtherActor))
    (if (not (`Pawn.IsPlayerControlled` _asbp_character_player))
      (`self.SetActorTickEnabled` true)
      (`PrimitiveComponent.SetCollisionResponseToChannel` (`self.BoxCollision`) "ECC_Pawn" "ECR_Overlap"))))

(event `self.ReceiveTick`
  (params (DeltaSeconds :type "Float (single-precision)"))
  (bind _boxcollision (`self.BoxCollision`))
  (bind _invertaxis (`self.InvertAxis`))
  (bind _boxcollision_2 (`self.BoxCollision`))
  (bind _returnvalue (`SceneComponent.GetForwardVector` _boxcollision))
  (bind _returnvalue_2 (`SceneComponent.GetRightVector` _boxcollision))
  (bind _overlappingactors (`PrimitiveComponent.GetOverlappingActors` (`self.BoxAI`) "/Game/Game/Actors/Characters/BP_Character_Player.BP_Character_Player_C"))
  (bind _returnvalue_3 (select `bool` _invertaxis :`false` -100 :`true` 100))
  (bind _returnvalue_4 (select `bool` _invertaxis :`false` 100 :`true` -100))
  (if (== (`KismetArrayLibrary.Array_Length` _overlappingactors) 0)
    (`self.SetActorTickEnabled` false)
    (`PrimitiveComponent.SetCollisionResponseToChannel` (`self.BoxCollision`) "ECC_Pawn" "ECR_Block")
    (else
      (for _array_element (`PrimitiveComponent.GetOverlappingActors` (`self.BoxCollision`) "/Game/Game/Actors/Characters/BP_Character_Player.BP_Character_Player_C")
        (bind _asbp_character_player (cast `/Game/Game/Actors/Characters/BP_Character_Player` _array_element))
        (if (`Pawn.IsPlayerControlled` _asbp_character_player)
          (bind _charactermovement (`Character.CharacterMovement` _asbp_character_player))
          (set `MovementComponent.Velocity` (0.0 0.0 0.0) _charactermovement)
          (`CharacterMovementComponent.AddImpulse` _charactermovement (`KismetMathLibrary.MakeVector` (.x (select `bool` (`self.X Or Y`) :`false` (select `bool` (> (.y (`KismetMathLibrary.InverseTransformDirection` (`SceneComponent.K2_GetComponentToWorld` _boxcollision_2) (`KismetMathLibrary.Normal` (- (`SceneComponent.K2_GetComponentLocation` (`Character.CapsuleComponent` _asbp_character_player)) (`SceneComponent.K2_GetComponentLocation` _boxcollision_2))))) 0.0) :`false` (* _returnvalue_2 _returnvalue_3) :`true` (* _returnvalue_2 _returnvalue_4)) :`true` (select `bool` (> (.x (`KismetMathLibrary.InverseTransformDirection` (`SceneComponent.K2_GetComponentToWorld` _boxcollision_2) (`KismetMathLibrary.Normal` (- (`SceneComponent.K2_GetComponentLocation` (`Character.CapsuleComponent` _asbp_character_player)) (`SceneComponent.K2_GetComponentLocation` _boxcollision_2))))) 0.0) :`false` (* _returnvalue _returnvalue_3) :`true` (* _returnvalue _returnvalue_4)))) (.y (select `bool` (`self.X Or Y`) :`false` (select `bool` (> (.y (`KismetMathLibrary.InverseTransformDirection` (`SceneComponent.K2_GetComponentToWorld` _boxcollision_2) (`KismetMathLibrary.Normal` (- (`SceneComponent.K2_GetComponentLocation` (`Character.CapsuleComponent` _asbp_character_player)) (`SceneComponent.K2_GetComponentLocation` _boxcollision_2))))) 0.0) :`false` (* _returnvalue_2 _returnvalue_3) :`true` (* _returnvalue_2 _returnvalue_4)) :`true` (select `bool` (> (.x (`KismetMathLibrary.InverseTransformDirection` (`SceneComponent.K2_GetComponentToWorld` _boxcollision_2) (`KismetMathLibrary.Normal` (- (`SceneComponent.K2_GetComponentLocation` (`Character.CapsuleComponent` _asbp_character_player)) (`SceneComponent.K2_GetComponentLocation` _boxcollision_2))))) 0.0) :`false` (* _returnvalue _returnvalue_3) :`true` (* _returnvalue _returnvalue_4)))) 5.0) true)
          (elif (`self.Jump`)
            (`Character.Jump` _asbp_character_player))))
      (set `self.ai` 0)
      (for _array_element_2 _overlappingactors
        (bind _asbp_character_player_2 (cast `/Game/Game/Actors/Characters/BP_Character_Player` _array_element_2))
        (if (`Pawn.IsBotControlled` _asbp_character_player_2)
          (`/Engine/EditorBlueprintResources/StandardMacros.IncrementInt` (`self.ai`)
            (:`  `
              (break)))))
      (if (== (`self.ai`) 0)
        (`self.SetActorTickEnabled` false)
        (`PrimitiveComponent.SetCollisionResponseToChannel` (`self.BoxCollision`) "ECC_Pawn" "ECR_Block")))))

(event `self.ReceiveBeginPlay`
  (bind _output (`|ConvertAsset` (`self.Parent`)))
  (if (not (`self.Enabled`))
    (`self.Func_Toggle`))
  (if (`KismetSystemLibrary.IsValid` _output)
    (add `self.DispatchEnabled` _output (delegate `ParentEnabled`))))

(event `ParentEnabled` :!signature `self.DispatchEnabled`
  (params (Enabled :type Boolean))
  (set `self.Enabled` Enabled))

(fn `Func_SetAIBox`
  (bind _boxai (`self.BoxAI`))
  (bind _boxcollision (`self.BoxCollision`))
  (bind _extraaisize (`self.ExtraAISize`))
  (`BoxComponent.SetBoxExtent` _boxai (+ (`BoxComponent.GetUnscaledBoxExtent` _boxcollision) (`KismetMathLibrary.MakeVector` _extraaisize _extraaisize _extraaisize)) true)
  (`SceneComponent.K2_SetRelativeTransform` _boxai (`KismetMathLibrary.MakeTransform` (.location (`SceneComponent.GetRelativeTransform` _boxcollision)) (.rotation (`SceneComponent.GetRelativeTransform` _boxcollision)) (.scale (`SceneComponent.GetRelativeTransform` _boxcollision))) false false))

(fn `Func_Toggle`
  (bind _staticmesh (`self.StaticMesh`))
  (bind _staticmesh_2 (`self.StaticMesh`))
  (if (`self.Enabled`)
    (`PrimitiveComponent.SetCollisionResponseToChannel` (`self.BoxCollision`) "ECC_Pawn" "ECR_Block")
    (`SceneComponent.SetVisibility` _staticmesh true false)
    (`PrimitiveComponent.SetCollisionEnabled` _staticmesh "QueryAndPhysics")
    (else
      (`self.SetActorTickEnabled` false)
      (`PrimitiveComponent.SetCollisionResponseToChannel` (`self.BoxCollision`) "ECC_Pawn" "ECR_Ignore")
      (`SceneComponent.SetVisibility` _staticmesh_2 false false)
      (`PrimitiveComponent.SetCollisionEnabled` _staticmesh_2 "NoCollision")))
  (return))

(fn `OnRep_Enabled`
  (`self.Func_Toggle`)
  (`self.DispatchEnabled` (`self.Enabled`))
  (return))

(fn `UserConstructionScript`
  (`StaticMeshComponent.SetStaticMesh` (`self.StaticMesh`) (`self.StaticMeshType`))
  (`self.Func_SetAIBox`))