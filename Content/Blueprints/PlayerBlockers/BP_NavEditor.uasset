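; BP_NavEditor is a level-placed actor that swaps nav area classes inside its box bounds at runtime in multiplayer modes.
; On authority, it waits for asset loading, then binds to objective activation, owner change or counterattack, or without an objective applies the new area by scenario.
; Round starts can also set either area.
; Delayed changes hit every RecastNavMesh, using tile-bounds replacement in TileMode or location-based change otherwise, with test and undo events.
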(event `self.ReceiveBeginPlay`
  ;[1 1 1] Init
  (`/Engine/EditorBlueprintResources/ActorMacros.Switch Has Authority`
    (:`Authority`
      (bind _asinsmultiplayer_mode (cast `INSMultiplayerMode` (`GameplayStatics.GetGameMode`) :!label _label)
        (:`then`
          (set `self.Gamemode` _asinsmultiplayer_mode)
          (if (== (`GameMode.GetMatchState` _asinsmultiplayer_mode) "LoadingAssets")
            (`KismetSystemLibrary.K2_SetTimerDelegate` (delegate `Safe Load`) 0.2 :!label _label_2)
            (else
              (`self.Init`))))
        (:`CastFailed`
          (goto _label_2))))))

(event `Safe Load`
  ;[1 1 1] Init
  (goto _label))

(event `Init`
  (bind _output (`|ConvertAsset` (`self.UseObjective`)))
  (`|ExecutionSequence`
    (:`then_0`
      ;[1 1 1] If objective is set then use Objective mode behaviour
      (if (`KismetSystemLibrary.IsValid` (`|ConvertAsset` (`self.UseObjective`)))
        (`KismetSystemLibrary.Delay` 0.1)
        (`|ExecutionSequence`
          (:`then_0`
            (if (or (`self.OnActive1`) (`self.OnActive0`))
              (add `ObjectiveBase.OnObjectiveActiveDelegate` _output (delegate `OnObjectiveActiveDelegate_Event_0`))))
          (:`then_1`
            (if (or (`self.OnNewOwner`) (`self.OnCounterAttack`))
              (add `ObjectiveBase.OnObjectiveChangeOwnerDelegate` _output (delegate `OnObjectiveChangeOwnerDelegate_Event_0`)))))
        (else
          ;[1 1 1] Clear scenarios and objective to set new area by default (for testing)
          (for _array_element (`self.Scenarios`)
            (set `self.RunByDefault` false)
            (bind _output_2 (`|ConvertAsset` _array_element))
            (if (`KismetSystemLibrary.IsValid` _output_2)
              (if (== _output_2 (`INSGameMode.Scenario` (`self.Gamemode`)))
                ;;[1 1 1] If scenario is set then it needs to be the active one
                (set `self.RunByDefault` true)
                (break))))
          (if (`self.RunByDefault`)
            (`self.SetNewArea`)))))
    (:`then_1`
      (if (or (`self.OnRoundStartNew`) (`self.OnRoundStartOld`))
        (add `INSMultiplayerMode.OnRoundActiveDelegate` (`self.Gamemode`) (delegate `OnRoundActiveDelegate_Event_0`))))))

(event `SetNewArea`
  (bind _newarea (`self.NewArea`))
  (bind (_origin _boxextent) (`KismetSystemLibrary.GetComponentBounds` (`self.Box`)))
  ;[1 1 1] Set New Area
  (`KismetSystemLibrary.Delay` (+ (`self.Delay`) 0.01))
  (bind _outactors (`GameplayStatics.GetAllActorsOfClass` "/Script/NavigationSystem.RecastNavMesh" :!label _label_3))
  (for _array_element _outactors
    (if (`self.Tile Mode`)
      (`RecastNavMesh.K2_ReplaceAreaInTileBounds` _array_element (`KismetMathLibrary.MakeBox` (- _origin _boxextent) (+ _origin _boxextent)) (`self.OldArea`) _newarea (`self.Replace Links (Tile)`))
      (else
        (`INSAIBlueprintLibrary.ChangeNavAreaAtLocation` _array_element _origin _boxextent _newarea)))))

(event `Test (Tile Mode)`
  ;[1 1 1] Set New Area
  (goto _label_3))

(event `OnObjectiveActiveDelegate_Event_0`
  (params (bNewActiveState :type Boolean) (Objective :type "ObjectiveBase Object Reference"))
  (if bNewActiveState
    (if (`self.OnActive1`)
      (`self.SetNewArea`))
    (elif (`self.OnActive0`)
      (`self.SetOldArea`))))

(event `OnObjectiveChangeOwnerDelegate_Event_0`
  (params (Objective :type "ObjectiveBase Object Reference") (NewOwners :type Byte))
  (bind _gamemode (`self.Gamemode`))
  (`|ExecutionSequence`
    (:`then_0`
      (if (`self.OnNewOwner`)
        (if (== NewOwners (select `bool` (`self.newOwnerIsAttacker`) :`false` (`INSGameMode.GetDefendingTeam` _gamemode) :`true` (`INSGameMode.GetAttackingTeam` _gamemode)))
          (`self.SetNewArea`))))
    (:`then_1`
      (if (`self.OnCounterAttack`)
        (if (and (`ObjectiveBase.GetActive` Objective) (`ObjectiveBase.bCounterAttack` Objective))
          (`self.SetNewArea`))))))

(event `Undo  (Tile Mode)`
  (bind _oldarea (`self.OldArea`))
  (bind (_origin _boxextent) (`KismetSystemLibrary.GetComponentBounds` (`self.Box`)))
  ;[1 1 1] Set Old Area
  (bind _outactors (`GameplayStatics.GetAllActorsOfClass` "/Script/NavigationSystem.RecastNavMesh" :!label _label_4))
  (for _array_element _outactors
    (if (`self.Tile Mode`)
      (`RecastNavMesh.K2_ReplaceAreaInTileBounds` _array_element (`KismetMathLibrary.MakeBox` (- _origin _boxextent) (+ _origin _boxextent)) (`self.NewArea`) _oldarea (`self.Replace Links (Tile)`))
      (else
        (`INSAIBlueprintLibrary.ChangeNavAreaAtLocation` null _origin _boxextent _oldarea)))))

(event `SetOldArea`
  ;[1 1 1] Set Old Area
  (`KismetSystemLibrary.Delay` (`self.Delay`))
  (goto _label_4))

(event `OnRoundActiveDelegate_Event_0`
  (`|ExecutionSequence`
    (:`then_0`
      (if (`self.OnRoundStartNew`)
        (`self.SetNewArea`)))
    (:`then_1`
      (if (`self.OnRoundStartOld`)
        (`self.SetOldArea`)))))

(fn `UserConstructionScript`)