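; Server-driven manager for the KWI Operation gamemode, running randomized objectives, supply crates and extraction.
; It randomly picks "real" locations, moving the gamemode's capturable objective onto one when discovered or overlapped.
; Stage changes hand objectives to defenders and relocate their spawns to nearby player starts; extraction adds music cues and a timer sprinting enemy bots to the objective.
; Non-dedicated instances poll to inject the Operation widget into tactical maps.
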(event `OnRoundActive`
  (bind _returnvalue (`INSGameMode.GetFirstActiveObjective` (`self.Gamemode`)))
  ;[0.329 1 0] OnRoundActive
  (set `self.CurrentSurvivalObjective` null)
  (`KismetSystemLibrary.Delay` 0.5)
  (if (`KismetSystemLibrary.IsValid` _returnvalue) :!label _label
    (bind _output_get (set `self.CurrentSurvivalObjective` _returnvalue))
    (if (!= (`INSSurvivalGameMode.NumWaves` (`self.Gamemode`)) 1)
      (`ObjectiveBase.SetObjectiveActive` _output_get false)
      (else
        (clear `ObjectiveBase.OnObjectiveChangeCapturingTeamDelegate` _output_get)
        (add `ObjectiveBase.OnObjectiveChangeCapturingTeamDelegate` _output_get (`|CreateDelegate` :!event `OnOwnerChangedFinal`))))
    (`self.MakeObjectivesMobile`)
    (`self.ResetLocations`)
    (set `self.CompletedObjectives` 0)
    (`self.CancelFinalBots`)
    (else
      (`KismetSystemLibrary.K2_SetTimerDelegate` (delegate `WaitForObjective`) 1.0))))

(event `OnPreRoundActive`
  ;[0.04235 0.2958 1] OnPreRound Music Events
)

(event `OnOwnerChangedFinal`
  (params (Objective :type "ObjectiveBase Object Reference") (NewOwners :type Byte))
  (bind _gamemode (`self.Gamemode`))
  ;[0.04235 0.2958 1] OnDefend Music Events
  (if (== NewOwners (`self.DefendingTeam`))
    (`|ExecutionSequence`
      (:`then_0`
        (for _array_element (`self.Crates_Permanent`)
          (set `/CustomScenario/Blueprints/Operation/BP_Operation_LimitedCrate.Discovered` true _array_element)))
      (:`then_1`
        (`INSGameMode.BroadcastMusicEvent` _gamemode "MoveToExtraction")
        (`KismetSystemLibrary.Delay` 1.0)
        (if (`INSMultiplayerMode.IsRoundRunning` _gamemode)
          (`INSGameMode.BroadcastMusicEvent` _gamemode "DefendExtractionPoint"))))))

(event `OnRoundOver`
  (params (RoundEndReason :type "ERoundConclusion Enum" :default "Generic") (WinningTeam :type Byte))
  (if (!= WinningTeam (`self.DefendingTeam`))
    (for _array_element (`self.ObjectiveLocations`)
      (if (`KismetSystemLibrary.IsPackagedForDistribution`)
        (set `/CustomScenario/Blueprints/Operation/BP_OPERATION_ObjectiveLocation.Discovered` false _array_element)
        (else
          (set `/CustomScenario/Blueprints/Operation/BP_OPERATION_ObjectiveLocation.Discovered` (`self.EditorDiscovered`) _array_element))))))

(event `WaitForObjective`
  ;[0.329 1 0] OnRoundActive
  (goto _label))

(event `FinalBots`)

(event `CustomEvent_2`
  (params (Objective :type "ObjectiveBase Object Reference") (NewOwners :type Byte))
  (bind _newvar_0 (`self.NewVar_0`))
  (`KismetSystemLibrary.Delay` 0.2)
  (`self.CancelFinalBots`)
  (if (== NewOwners (`self.DefendingTeam`))
    (bind _outactors (`GameplayStatics.GetAllActorsOfClass` "/Script/Insurgency.INSAISoldierController"))
    (`KismetArrayLibrary.Array_Clear` (`self.HostileBots`))
    (for _array_element _outactors
      (if (== (`self.AttackingTeam`) (`INSAISoldierController.GetTeamId` _array_element))
        (`KismetArrayLibrary.Array_AddUnique` (`self.HostileBots`) _array_element)))
    (if (`KismetSystemLibrary.K2_IsValidTimerHandle` _newvar_0)
      (`KismetSystemLibrary.K2_ClearAndInvalidateTimerHandle` _newvar_0))
    (bind _returnvalue (`KismetSystemLibrary.K2_SetTimer` null "SprintBotsFinal" 0.2 true))
    (set `self.NewVar_0` _returnvalue)))

(event `CustomEvent_1`
  (params (ObjetiveLocation :type "/CustomScenario/Blueprints/Operation/BP_OPERATION_ObjectiveLocation Object Reference") (`New Checked` :type Boolean))
  ;[1 1 1] Discovery
  (if `New Checked`
    (`self.MoveObjective` ObjetiveLocation true)))

(event `Enable Real`
  ;[1 1 1] Enable our picked objectives
  (for _array_element (`self.RealLocations`)
    (set `/CustomScenario/Blueprints/Operation/BP_OPERATION_ObjectiveLocation.Real` true _array_element))
  (`self.RefreshAllOnClients`))

(event `OnObjectiveOverlap`
  (params (ObjectiveLocation :type "/CustomScenario/Blueprints/Operation/BP_OPERATION_ObjectiveLocation Object Reference") (INSSoldier :type "INSSoldier Object Reference"))
  ;[1 1 1] Discovery
  (if (not (`/CustomScenario/Blueprints/Operation/BP_OPERATION_ObjectiveLocation.Discovered` ObjectiveLocation))
    (set `/CustomScenario/Blueprints/Operation/BP_OPERATION_ObjectiveLocation.Discovered` true ObjectiveLocation))
  (`self.MoveObjective` ObjectiveLocation))

(event `CancelFinalBots`
  (`KismetSystemLibrary.K2_ClearAndInvalidateTimerHandle` (`self.NewVar_0`)))

(event `Rebind Events`
  ;[1 1 1] Rebind Objective Events
  (for _array_element (`self.ObjectiveLocations`)
    (clear `/CustomScenario/Blueprints/Operation/BP_OPERATION_ObjectiveLocation.StageStateChanged` _array_element)
    (clear `/CustomScenario/Blueprints/Operation/BP_OPERATION_ObjectiveLocation.DiscoveredStateChanged` _array_element))
  (for _array_element_2 (`self.RealLocations`)
    (add `/CustomScenario/Blueprints/Operation/BP_OPERATION_ObjectiveLocation.StageStateChanged` _array_element_2 (`|CreateDelegate` :!event `OnStageUpdate`))))

(event `WaitGetActiveObjective`
  ;[1 1 1] Wait Get Active Objective
  (`KismetSystemLibrary.Delay` 0.1)
  (`self.GetActiveObjective`))

(event `Recheck`
  (bind _reallocations (`self.RealLocations`))
  (bind _returnvalue (`KismetArrayLibrary.Array_Length` (`self.RealLocations`)))
  (bind _returnvalue_2 (- (`self.numWaves`) 1))
  (bind _output (`|GetArrayItem` (`self.ObjectiveLocations`) (`self.StoredRandom`)))
  ;[1 1 1] Temp objective randomizer
  (if (< _returnvalue _returnvalue_2)
    (`KismetSystemLibrary.PrintString` (`KismetStringLibrary.Concat_StrStr` "Recheck Length: " (`KismetStringLibrary.Conv_IntToString` _returnvalue) " Wanted: " (`KismetStringLibrary.Conv_IntToString` _returnvalue_2)) false false)
    (set `self.StoredRandom` (`KismetMathLibrary.RandomIntegerInRange` 0 (`KismetArrayLibrary.Array_LastIndex` (`self.ObjectiveLocations`))))
    (if (`KismetArrayLibrary.Array_Contains` _reallocations _output)
      _
      (elif (`/CustomScenario/Blueprints/Operation/BP_OPERATION_ObjectiveLocation.Initialized` _output)
        (`KismetArrayLibrary.Array_AddUnique` _reallocations _output)))
    (`KismetSystemLibrary.K2_SetTimerDelegate` (delegate `Recheck`) 0.01)
    (else
      (`KismetSystemLibrary.PrintString` "Done Checking" false false)
      (`self.Enable Real`)
      (`self.Rebind Events`))))

(event `self.ReceiveBeginPlay`
  (bind _gamemode (`self.Gamemode`))
  (bind _reallocations (`self.RealLocations`))
  (bind _objectivelocations (`self.ObjectiveLocations`))
  (bind _output (`|GetArrayItem` (`self.ObjectiveLocations`) (`self.StoredRandom`)))
  (if (`KismetSystemLibrary.IsServer`)
    (`|ExecutionSequence`
      (:`then_0`
        ;[1 0 0.7039] Only Server
        (`|ExecutionSequence`
          (:`then_0`
            (bind _askwioperation_gamemode (cast `/CustomScenario/Blueprints/Operation/KWIOperationGamemode` (`GameplayStatics.GetGameMode`)))
            (if (`KismetSystemLibrary.IsPackagedForDistribution`)
              _
              (elif false
                (`INSGameMode.SetPropertyValueFromFloat` _askwioperation_gamemode "PreRoundTIme" 1.0)
                (`INSGameMode.SetPropertyValueFromFloat` _askwioperation_gamemode "ExtractionObjectiveHoldTime" 45.0)))
            (set `self.Gamemode` _askwioperation_gamemode)
            (set `self.DefendingTeam` (`INSGameMode.GetDefendingTeam` _askwioperation_gamemode))
            (set `self.AttackingTeam` (`INSGameMode.GetAttackingTeam` _askwioperation_gamemode))
            (bind _output_get (set `self.numWaves` (`INSSurvivalGameMode.NumWaves` _askwioperation_gamemode)))
            ;[1 1 1] OnRound binds
            (`KismetSystemLibrary.PrintString` (`KismetStringLibrary.Concat_StrStr` "Waves: " (`KismetStringLibrary.Conv_IntToString` _output_get)) false false)
            (add `INSMultiplayerMode.OnRoundActiveDelegate` _gamemode (`|CreateDelegate` :!event `OnRoundActive`))
            (add `INSMultiplayerMode.OnPreRoundStartedDelegate` _gamemode (`|CreateDelegate` :!event `OnPreRoundActive`))
            (add `INSMultiplayerMode.OnRoundOverDelegate` _gamemode (`|CreateDelegate` :!event `OnRoundOver`)))
          (:`then_1`
            (bind _outactors (`GameplayStatics.GetAllActorsOfClass` "/CustomScenario/Blueprints/Operation/BP_OPERATION_ObjectiveLocation.BP_Operation_ObjectiveLocation_C"))
            (bind _output_get_2 (set `self.ObjectiveLocations` _outactors))
            (for _array_element _output_get_2
              ;[1 1 1] Discovery
              (add `/CustomScenario/Blueprints/Operation/BP_OPERATION_ObjectiveLocation.PlayerOverlap` _array_element (`|CreateDelegate` :!event `OnObjectiveOverlap`))
              (set `/CustomScenario/Blueprints/Operation/BP_OPERATION_ObjectiveLocation.Real` false _array_element)
              (add `/CustomScenario/Blueprints/Operation/BP_OPERATION_ObjectiveLocation.DiscoveredStateChanged` _array_element (delegate `CustomEvent_1`))))
          (:`then_2`
            ;[1 1 1] Temp objective randomizer
            (if (`KismetArrayLibrary.Array_IsValidIndex` _objectivelocations)
              (for _ (range (+ (`KismetMathLibrary.Clamp` (- (`self.numWaves`) 2) 0 9999) 1))
                (set `self.StoredRandom` (`KismetMathLibrary.RandomIntegerInRange` 0 (`KismetArrayLibrary.Array_LastIndex` _objectivelocations)))
                (if (`KismetArrayLibrary.Array_Contains` _reallocations _output)
                  _
                  (elif (`/CustomScenario/Blueprints/Operation/BP_OPERATION_ObjectiveLocation.Initialized` _output)
                    (`KismetArrayLibrary.Array_AddUnique` _reallocations _output))))
              (`self.Recheck`)))
          (:`then_3`
            (`self.CrateRand`))))
      (:`then_1`
        ;[1 0.04957 0.7413] Offline player
        (if (not (`KismetSystemLibrary.IsDedicatedServer`))
          ;[1 0.2743 0] Offline + Clients Init
          (`|ExecutionSequence` :!label _label_2
            (:`then_0`
              ;[1 1 1] Inject Map Widget
              (`KismetSystemLibrary.K2_SetTimerDelegate` (delegate `CustomEvent_0`) 1.0 true))))))
    (else
      (goto _label_2))))

(event `MakeObjectivesMobile`
  ;[1 1 1] Make Objectives Mobile
  (bind _outactors (`GameplayStatics.GetAllActorsOfClass` "/Script/Insurgency.ObjectiveCapturable"))
  (for _array_element _outactors
    (bind _asbox_collision (cast `BoxComponent` (`Actor.RootComponent` _array_element)))
    (`SceneComponent.SetMobility` _asbox_collision "Movable")))

(event `MoveObjective`
  (params (ObjetiveLocation :type "/CustomScenario/Blueprints/Operation/BP_OPERATION_ObjectiveLocation Object Reference") (Discovered :type Boolean))
  (bind _currentsurvivalobjective (`self.CurrentSurvivalObjective`))
  ;[1 1 1] Move Objective
  (if Discovered
    (`ObjectiveBase.SetObjectiveActive` _currentsurvivalobjective true :!label _label_3)
    (`self.ReplicatedMoveObjective1` _currentsurvivalobjective ObjetiveLocation)
    (elif (and (== (`/CustomScenario/Blueprints/Operation/BP_OPERATION_ObjectiveLocation.ObjectiveStage` ObjetiveLocation) 0) (`/CustomScenario/Blueprints/Operation/BP_OPERATION_ObjectiveLocation.Initialized` ObjetiveLocation) (`/CustomScenario/Blueprints/Operation/BP_OPERATION_ObjectiveLocation.ObjectiveActive` ObjetiveLocation) (`/CustomScenario/Blueprints/Operation/BP_OPERATION_ObjectiveLocation.Real` ObjetiveLocation))
      (goto _label_3))))

(event `OnStageUpdate`
  (params (ObjectiveLocation :type "/CustomScenario/Blueprints/Operation/BP_OPERATION_ObjectiveLocation Object Reference") (`New Stage` :type Byte))
  ;[1 1 1] On StaGe Changed
  (`KismetSystemLibrary.PrintString` (`KismetStringLibrary.Conv_ByteToString` `New Stage`) false false)
  (switch `int` (`KismetMathLibrary.Conv_ByteToInt` `New Stage`)
    (:`Default`
      (if (== `New Stage` 1)
        (`self.Progress Objective`)))))

(event `CustomEvent_0`
  ;[1 1 1] Inject Map Widget
  (bind _foundwidgets (`WidgetBlueprintLibrary.GetAllWidgetsOfClass` "/Game/UI/Widgets/HUD/TacticalMap/BP_Widget_TacticalMap_Native.BP_Widget_TacticalMap_Native_C" false))
  (for _array_element _foundwidgets
    (bind _returnvalue (`Widget.GetParent` (`/Game/UI/Widgets/HUD/TacticalMap/BP_Widget_TacticalMap_Native.GridInvalidationBox` _array_element)))
    (bind _isspawned (`self.CheckIfSpawnedWidget` _returnvalue))
    (if (not _isspawned)
      (bind _returnvalue_2 (`|CreateWidget` "/CustomScenario/Blueprints/Operation/BP_Widget_Operation.BP_Widget_Operation_C" (`GameplayStatics.GetPlayerController` 0)))
      (`PanelWidget.AddChild` _returnvalue _returnvalue_2))))

(event `MoveSpawnZone`
  (params (SpawnZone :type "SpawnZone Object Reference") (Transform :type "Transform Structure"))
  ;[1 1 1] Replicated move spawnzone
  (`SceneComponent.SetMobility` (`Actor.RootComponent` SpawnZone) "Movable")
  (`self.K2_SetActorTransform` Transform)
  (`KismetSystemLibrary.PrintString` "Moved" true true (struct :`R` 1.0 :`G` 0.120504 :`A` 1.0) 8.0))

(event `ReplicatedMoveObjective1`
  (params (`Objective Base` :type "ObjectiveBase Object Reference") (ObjectiveLocation :type "/CustomScenario/Blueprints/Operation/BP_OPERATION_ObjectiveLocation Object Reference"))
  ;[1 1 1] Replicated Move Objective
  (bind _asbox_collision (cast `BoxComponent` (`Actor.RootComponent` `Objective Base`)))
  (`SceneComponent.SetMobility` _asbox_collision "Movable")
  (`PrimitiveComponent.SetCollisionEnabled` _asbox_collision "NoCollision")
  (`self.K2_SetActorTransform` `Objective Base` (`self.GetTransform` ObjectiveLocation) false false))

(event `RefreshAllOnClients`
  ;[1 1 1] Refresh client widget
  (if (not (`KismetSystemLibrary.IsDedicatedServer`))
    (bind _foundwidgets (`WidgetBlueprintLibrary.GetAllWidgetsOfClass` "/CustomScenario/Blueprints/Operation/BP_Widget_Operation.BP_Widget_Operation_C" false))
    (for _array_element _foundwidgets
      (`/CustomScenario/Blueprints/Operation/BP_Widget_Operation.RefreshAll` _array_element))))

(fn `CheckIfSpawnedWidget`
  (params (`Parent Widget` :type "PanelWidget Object Reference"))
  (returns (IsSpawned :type Boolean))
  (locals (IsSpawnedLocal :type Boolean :default false))
  (for _array_element (`PanelWidget.GetAllChildren` `Parent Widget`)
    (if (== (`GameplayStatics.GetObjectClass` _array_element) "/CustomScenario/Blueprints/Operation/BP_Widget_Operation.BP_Widget_Operation_C")
      (set `local.IsSpawnedLocal` true)
      (break)))
  (return (`local.IsSpawnedLocal`)))

(fn `CrateRand`
  (locals (UseFullRandom :type Boolean :default false) (InitilizedCrates :type Integer))
  (bind _initilizedcrates (`local.InitilizedCrates`))
  (bind _cratemax (`/CustomScenario/Blueprints/Operation/KWIOperationGamemode.CrateMax` (`self.Gamemode`)))
  (bind _outactors (`GameplayStatics.GetAllActorsOfClass` "/CustomScenario/Blueprints/Operation/BP_Operation_LimitedCrate.BP_Operation_LimitedCrate_C"))
  (bind _output_get (set `self.Crates` _outactors))
  (bind _returnvalue (`KismetArrayLibrary.Array_Length` _outactors))
  (set `local.UseFullRandom` (> _cratemax _returnvalue))
  (set `self.CrateMax` (`KismetMathLibrary.Clamp` _cratemax 0 _returnvalue))
  (`KismetArrayLibrary.Array_Shuffle` _output_get)
  (set `local.InitilizedCrates` 0)
  (for _array_element _output_get
    (if (`/CustomScenario/Blueprints/Operation/BP_Operation_LimitedCrate.AlwaysActive` _array_element)
      (set `/CustomScenario/Blueprints/Operation/BP_Operation_LimitedCrate.Initialized` true _array_element)
      (`/CustomScenario/Blueprints/Operation/BP_Operation_LimitedCrate.Initilize` _array_element)
      (`KismetArrayLibrary.Array_AddUnique` (`self.Crates_Permanent`) _array_element)
      (elif (`local.UseFullRandom`)
        (if (<= (`KismetMathLibrary.RandomFloat`) (`/CustomScenario/Blueprints/Operation/KWIOperationGamemode.CrateRand` (`self.Gamemode`)))
          (`/Engine/EditorBlueprintResources/StandardMacros.IncrementInt` _initilizedcrates
            (:`  `
              (set `/CustomScenario/Blueprints/Operation/BP_Operation_LimitedCrate.Initialized` true _array_element)
              (`/CustomScenario/Blueprints/Operation/BP_Operation_LimitedCrate.Initilize` _array_element))))
        (elif (< (`local.InitilizedCrates`) (`self.CrateMax`))
          (`/Engine/EditorBlueprintResources/StandardMacros.IncrementInt` _initilizedcrates
            (:`  `
              (set `/CustomScenario/Blueprints/Operation/BP_Operation_LimitedCrate.Initialized` true _array_element)
              (`/CustomScenario/Blueprints/Operation/BP_Operation_LimitedCrate.Initilize` _array_element)))
          (else
            (break))))))
  (`KismetSystemLibrary.PrintString` (`KismetStringLibrary.Concat_StrStr` "Initilized Crates: " (`KismetStringLibrary.Conv_IntToString` (`local.InitilizedCrates`)) " / " (`KismetStringLibrary.Conv_IntToString` _returnvalue))))

(fn `GetActiveObjective`
  (bind _currentsurvivalobjective (`self.CurrentSurvivalObjective`))
  (bind _outobjectives (`INSGameMode.GetActiveObjectives` (`self.Gamemode`)))
  (bind _output (`|GetArrayItem` _outobjectives (`KismetArrayLibrary.Array_LastIndex` _outobjectives)))
  (if (`KismetArrayLibrary.Array_IsValidIndex` _outobjectives)
    (if (!= _output (`self.CurrentSurvivalObjective`))
      (bind _output_get (set `self.CurrentSurvivalObjective` _output))
      (if (not (< (`self.CompletedObjectives`) (- (`self.numWaves`) 1)))
        (clear `ObjectiveBase.OnObjectiveChangeOwnerDelegate` _currentsurvivalobjective)
        (add `ObjectiveBase.OnObjectiveChangeOwnerDelegate` _currentsurvivalobjective (`|CreateDelegate` :!event `OnOwnerChangedFinal`)))
      (if (`self.NeedHideObjective`)
        (set `self.NeedHideObjective` false)
        (`ObjectiveBase.SetObjectiveActive` _output_get false))
      (return)
      (else
        (`self.WaitGetActiveObjective`)
        (return)))
    (else
      (`self.WaitGetActiveObjective`)
      (return))))

(fn `MoveSpawns`
  (params (ObjectiveBase :type "ObjectiveBase Object Reference"))
  (locals (min :type "Float (double-precision)" :default 7000.0) (Closest :type "/CustomScenario/Blueprints/Operation/BP_OperationPlayerStarts Object Reference") (closestvalue :type "Float (double-precision)" :default 99999997952.0))
  (bind _closest (`local.Closest`))
  (bind _outactors (`GameplayStatics.GetAllActorsOfClass` "/CustomScenario/Blueprints/Operation/BP_OperationPlayerStarts.BP_OperationPlayerStarts_C"))
  (set `local.Closest` null)
  (for _array_element _outactors :!label _label
    (bind _returnvalue (`self.GetDistanceTo` _array_element (`local.ObjectiveBase`)))
    (if (and (> _returnvalue (`local.min`)) (< _returnvalue (`local.closestvalue`)))
      (set `local.closestvalue` _returnvalue)
      (set `local.Closest` _array_element)))
  (if (`KismetSystemLibrary.IsValid` (`local.Closest`))
    (for _array_element_2 (`ObjectiveBase.AssociatedSpawnZones` (`local.ObjectiveBase`))
      (if (== (`SpawnZone.TeamId` _array_element_2) (`self.DefendingTeam`))
        (`self.MoveSpawnZone` _array_element_2 (`self.GetTransform` _closest))
        (for (_array_element_3 _array_index) (`SpawnZone.PlayerStarts` _array_element_2)
          (`SceneComponent.SetMobility` (`Actor.RootComponent` _array_element_3) "Movable")
          (bind _output (`|GetArrayItem` (`SceneComponent.GetChildrenComponents` (`Actor.RootComponent` _closest) false) _array_index))
          (if (`KismetSystemLibrary.IsValid` _output)
            (`self.K2_SetActorTransform` _array_element_3 (`SceneComponent.K2_GetComponentToWorld` _output) false false)
            (`self.K2_SetActorRotation` _array_element_3 (`KismetMathLibrary.Conv_VectorToRotator` (`KismetMathLibrary.Vector_Normal2D` (`/CustomScenario/Blueprints/Operation/BP_OperationPlayerStarts.LookAtMe` (`local.Closest`)))) false)))))
    (return)
    (elif (!= (`local.min`) 0.0)
      (set `local.min` (`KismetMathLibrary.FClamp` (- (`local.min`) 1000.0) 0.0 99999997952.0))
      (goto _label)
      (else
        (return)))))

(fn `Progress Objective`
  (bind _currentsurvivalobjective (`self.CurrentSurvivalObjective`))
  (bind _defendingteam (`self.DefendingTeam`))
  (bind _returnvalue (`INSMultiplayerMode.GetNumObjectivesOwnedForTeam` (`self.Gamemode`) (`self.DefendingTeam`) true))
  (bind _returnvalue_2 (`INSGameMode.GetFirstActiveObjective` (`self.Gamemode`)))
  (`KismetSystemLibrary.PrintString` (`KismetStringLibrary.Concat_StrStr` "Completed Objectives: " (`KismetStringLibrary.Conv_IntToString` _returnvalue)) false false (struct :`R` 1.0 :`G` 0.994406 :`B` 0.864183 :`A` 1.0))
  (if (< _returnvalue (`self.numWaves`))
    ;[1 1 1] Progress Objective
    (if (`KismetSystemLibrary.IsValid` _returnvalue_2)
      (`self.MoveSpawns` _returnvalue_2)
      (`ObjectiveBase.SetObjectiveActive` _returnvalue_2 true)
      (`ObjectiveBase.SetOwningTeam` _returnvalue_2 _defendingteam)
      (else
        (`self.MoveSpawns` (`self.CurrentSurvivalObjective`))
        (`ObjectiveBase.SetObjectiveActive` _currentsurvivalobjective true)
        (`ObjectiveBase.SetOwningTeam` _currentsurvivalobjective _defendingteam)))
    (bind _result (`/Engine/EditorBlueprintResources/StandardMacros.IncrementInt` (`self.CompletedObjectives`))
      (:`  `
        (bind _returnvalue_3 (< _result (- (`self.numWaves`) 1)))
        (set `self.NeedHideObjective` _returnvalue_3)
        (if _returnvalue_3
          (`self.GetActiveObjective`)
          (else
            (`self.GetActiveObjective`)))
        (return)))
    (else
      (return))))

(fn `ResetLocations`
  (for _array_element (`self.RealLocations`)
    (`/CustomScenario/Blueprints/Operation/BP_OPERATION_ObjectiveLocation.ProxyCleanup` _array_element)
    (`/CustomScenario/Blueprints/Operation/BP_OPERATION_ObjectiveLocation.ProxySetup` _array_element))
  (for _array_element_2 (`self.ObjectiveLocations`)
    (if (`KismetSystemLibrary.IsPackagedForDistribution`)
      (set `/CustomScenario/Blueprints/Operation/BP_OPERATION_ObjectiveLocation.Discovered` false _array_element_2)
      (else
        (set `/CustomScenario/Blueprints/Operation/BP_OPERATION_ObjectiveLocation.Discovered` (`self.EditorDiscovered`) _array_element_2))))
  (return))

(fn `SprintBotsFinal`
  (for _array_element (`self.HostileBots`)
    (if (`KismetSystemLibrary.IsValid` _array_element)
      (bind _returnvalue (`BotBehaviorHandler.GetActiveBehavior` (`INSAISoldierController.GetBehaviorHandler` _array_element)))
      (if (`KismetSystemLibrary.IsValid` _returnvalue)
        (if (!= (`GameplayStatics.GetObjectClass` _returnvalue) "/Script/Insurgency.BotBehavior_ClearObjective")
          (`INSAISoldierController.MoveToActorSafe` _array_element (`self.CurrentSurvivalObjective`) "Move to Objective" "Sprint" "Stand" "Important" false 300.0 false :!label _label))
        (else
          (goto _label)))))
  (return))

(fn `UserConstructionScript`)