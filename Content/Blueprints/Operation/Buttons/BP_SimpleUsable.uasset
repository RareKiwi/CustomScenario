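; BP_SimpleUsable is a basic usable actor that lets a pawn trigger use, completion and cancellation events.
; On authority it forwards each event to a dispatcher with a debug print, and its use handlers report server handling.
; Replicated EnabledUsable switches the Box between overlap and ignore on a game trace channel.
; RepNotify Parent and Offset reattach the actor to its parent at the relative transform.
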(event `OnUseEvent`
  (params (Pawn :type "INSSoldier Object Reference"))
  (`/Engine/EditorBlueprintResources/ActorMacros.Switch Has Authority`
    (:`Authority`
      (`self.OnUseDispatch` self Pawn)
      (`KismetSystemLibrary.PrintString` "OnUse"))))

(event `self.EventOnUseComplete`
  (params (Pawn :type "INSSoldier Object Reference"))
  (`/Engine/EditorBlueprintResources/ActorMacros.Switch Has Authority`
    (:`Authority`
      (`self.OnUseCompleteDispatch` self Pawn)
      (`KismetSystemLibrary.PrintString` "OnUseComplete"))))

(event `self.EventOnUseCancelled`
  (params (Pawn :type "INSSoldier Object Reference"))
  (`/Engine/EditorBlueprintResources/ActorMacros.Switch Has Authority`
    (:`Authority`
      (`self.OnUseCancelledDispatch` self Pawn)
      (`KismetSystemLibrary.PrintString` "OnUseCancelled"))))

(event `self.ReceiveBeginPlay`
  (`PrimitiveComponent.SetCollisionResponseToChannel` (`self.Box`) "ECC_GameTraceChannel4" (select `bool` (`self.EnabledUsable`) :`false` "ECR_Ignore" :`true` "ECR_Overlap" :!type "ECollisionResponse Enum")))

(event `AttachAndOffset`
  (if (`KismetSystemLibrary.IsValid` (`self.Parent`))
    (`self.K2_DetachFromActor` self "KeepWorld" "KeepWorld" "KeepWorld")
    (`self.K2_AttachToActor` (`self.Parent`) "None" "SnapToTarget" "SnapToTarget" "SnapToTarget")
    (`self.K2_SetActorRelativeTransform` (`self.Offset`))))

(fn `EventOnUseKeyReleased`
  (params (Pawn :type "INSSoldier Object Reference") (ElapsedTime :type "Float (double-precision)"))
  (returns (ReturnValue :type "EUseResponse Enum"))
  (return "HandledServer"))

(fn `EventTryUse`
  (params (Pawn :type "INSSoldier Object Reference") (HitResult :type "HitResult Structure (by ref)"))
  (returns (ReturnValue :type "EUseResponse Enum"))
  (if (`KismetSystemLibrary.IsValid` Pawn)
    (`self.OnUseEvent` Pawn)
    (return "HandledServer")
    (else
      (return "Ignore"))))

(fn `OnRep_EnabledUsable`
  (bind _enabledusable (`self.EnabledUsable`))
  (`PrimitiveComponent.SetCollisionResponseToChannel` (`self.Box`) "ECC_GameTraceChannel4" (select `bool` _enabledusable :`false` "ECR_Ignore" :`true` "ECR_Overlap" :!type "ECollisionResponse Enum"))
  (`KismetSystemLibrary.PrintString` (`KismetStringLibrary.Conv_BoolToString` _enabledusable))
  (return))

(fn `OnRep_Offset`
  (`self.AttachAndOffset`)
  (return))

(fn `OnRep_Parent`
  (`self.AttachAndOffset`)
  (return))

(fn `UserConstructionScript`)