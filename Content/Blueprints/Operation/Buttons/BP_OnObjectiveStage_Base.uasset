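; Base Blueprint, filed with operation buttons, that tracks the stage of a referenced objective operation and exposes changes to child classes.
; On authority, a looping timer polls for up to 20 seconds until the ObjectiveOperation reference is valid, then binds to its stage-change event.
; Each change sets ObjectiveStage, whose RepNotify calls the empty OnStageChangeRepNotify hook.
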(event `self.ReceiveBeginPlay`
  (`/Engine/EditorBlueprintResources/ActorMacros.Switch Has Authority`
    (:`Authority`
      (bind _returnvalue (`KismetSystemLibrary.K2_SetTimerDelegate` (delegate `Wait load`) 1.0 true))
      (`KismetSystemLibrary.Delay` 20.0)
      (`KismetSystemLibrary.K2_ClearAndInvalidateTimerHandle` _returnvalue))))

(event `Wait load`
  (if (`KismetSystemLibrary.IsValid` (`|ConvertAsset` (`self.ObjectiveOperation`)))
    (`KismetSystemLibrary.K2_ClearAndInvalidateTimerHandle` (stale `self.ReceiveBeginPlay` _returnvalue))
    (add `/CustomScenario/Blueprints/Operation/BP_OPERATION_ObjectiveLocation.StageStateChanged` (`|ConvertAsset` (`self.ObjectiveOperation`)) (delegate `OnStageChange`))))

(event `OnStageChange`
  (params (ObjectiveLocation :type "/CustomScenario/Blueprints/Operation/BP_OPERATION_ObjectiveLocation Object Reference") (`New Stage` :type Byte))
  (set `self.ObjectiveStage` `New Stage`))

(event `OnStageChangeRepNotify`
  (params (Stage :type Byte)))

(fn `OnRep_ObjectiveStage`
  (`self.OnStageChangeRepNotify` (`self.ObjectiveStage`))
  (return))

(fn `UserConstructionScript`)