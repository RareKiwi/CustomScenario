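; Objective-stage actor that shows an oil spill through a spreading decal and three particle systems, skipped on dedicated servers.
; The stage RepNotify hides effects at stage 0; stage 1 enables Tick, which interpolates the decal from Start to End, then stops and hides two particle systems, leaving the third.
; BeginPlay snaps to the finished spill when the stage is already set.
; ShowOil and Preview toggle particles and decal transform.
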(event `self.ReceiveBeginPlay`
  (bind _returnvalue (> (`self.ObjectiveStage`) 0))
  (`parent.ReceiveBeginPlay`)
  (if (not (`KismetSystemLibrary.IsDedicatedServer`))
    (`SceneComponent.SetVisibility` (`self.ParticleSystem`) false false)
    (`SceneComponent.SetVisibility` (`self.ParticleSystem1`) false false)
    (`SceneComponent.SetVisibility` (`self.Decal`) _returnvalue false)
    (`SceneComponent.SetVisibility` (`self.ParticleSystem2`) _returnvalue false)
    (if _returnvalue
      (`SceneComponent.K2_SetRelativeTransform` (`self.Decal`) (`self.End`) false false))))

(event `ShowOil`
  (bind _particlesystem (`self.ParticleSystem`))
  (`SceneComponent.SetVisibility` _particlesystem (not (`SceneComponent.bVisible` _particlesystem)) false)
  (`SceneComponent.SetVisibility` (`self.ParticleSystem1`) (not (`SceneComponent.bVisible` _particlesystem)) false)
  (`SceneComponent.SetVisibility` (`self.ParticleSystem2`) (not (`SceneComponent.bVisible` _particlesystem)) false))

(event `Preview`
  (if (`KismetMathLibrary.NearlyEqual_TransformTransform` (`SceneComponent.GetRelativeTransform` (`self.Decal`)) (`self.End`) 0.001 0.001 0.001)
    (`SceneComponent.K2_SetRelativeTransform` (`self.Decal`) (`self.Start`) false false)
    (else
      (`SceneComponent.K2_SetRelativeTransform` (`self.Decal`) (`self.End`) false false))))

(event `self.OnStageChangeRepNotify`
  (params (Stage :type Byte))
  (if (not (`KismetSystemLibrary.IsDedicatedServer`))
    (`SceneComponent.SetVisibility` (`self.Decal`) (> Stage 0) false)
    (switch `int` (`KismetMathLibrary.Conv_ByteToInt` Stage)
      (:`0`
        (`self.SetActorTickEnabled` false)
        (`SceneComponent.SetVisibility` (`self.ParticleSystem`) false false)
        (`SceneComponent.SetVisibility` (`self.ParticleSystem1`) false false)
        (`SceneComponent.SetVisibility` (`self.ParticleSystem2`) false false))
      (:`1`
        (`self.SetActorTickEnabled` true)
        (set `self.Current` (`self.Start`))
        (`SceneComponent.SetVisibility` (`self.ParticleSystem`) true false)
        (`SceneComponent.SetVisibility` (`self.ParticleSystem1`) true false)
        (`SceneComponent.SetVisibility` (`self.ParticleSystem2`) true false)))))

(event `self.ReceiveTick`
  (params (DeltaSeconds :type "Float (single-precision)"))
  (bind _returnvalue (`KismetMathLibrary.TInterpTo` (`self.Current`) (`self.End`) DeltaSeconds 0.3))
  (bind _output_get (set `self.Current` _returnvalue))
  (`SceneComponent.K2_SetRelativeTransform` (`self.Decal`) _output_get false false)
  (if (`KismetMathLibrary.NearlyEqual_TransformTransform` _returnvalue (`self.End`) 0.1 0.1 0.1)
    (`self.SetActorTickEnabled` false)
    (`SceneComponent.SetVisibility` (`self.ParticleSystem`) false false)
    (`SceneComponent.SetVisibility` (`self.ParticleSystem1`) false false)))

(fn `UserConstructionScript`
  (`SceneComponent.SetVisibility` (`self.ParticleSystem`) false false)
  (`SceneComponent.SetVisibility` (`self.ParticleSystem1`) false false)
  (`SceneComponent.SetVisibility` (`self.ParticleSystem2`) false false)
  (`parent.UserConstructionScript`))