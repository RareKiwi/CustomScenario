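; Operation-mode placeholder for a supply crate that the defending team discovers by walking into it.
; On the server, a defender's overlap marks it discovered and spawns a limited supply crate, or a base one if AlwaysActive.
; Round start destroys any spawned crate and resets discovery; replicated flags drive placeholder mesh visibility.
; AutoSize fits the box to surrounding geometry using six debug-drawn line traces along the AutoSizer's axes.
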(event `Auto Size`
  (`self.AutoSize`))

(event `Initilize`
  (if (`self.Initialized`) :!label _label
    (bind _askwioperation_gamemode (cast `/CustomScenario/Blueprints/Operation/KWIOperationGamemode` (`GameplayStatics.GetGameMode`)))
    (set `self.DefendingTeam` (`INSGameMode.GetDefendingTeam` _askwioperation_gamemode))
    (set `self.AttackingTeam` (`INSGameMode.GetAttackingTeam` _askwioperation_gamemode))
    (add `INSMultiplayerMode.OnRoundActiveDelegate` _askwioperation_gamemode (delegate `OnRoundActive`))
    (add `INSMultiplayerMode.OnRoundOverDelegate` _askwioperation_gamemode (delegate `OnRoundOverDelegate_Event_0`))
    (`self.UpdateVisibility`)))

(event `self.ReceiveBeginPlay`
  (`/Engine/EditorBlueprintResources/ActorMacros.Switch Has Authority`
    (:`Authority`
      (`self.UpdateVisibility`)
      (`KismetSystemLibrary.Delay` 1.0)
      (goto _label))
    (:`Remote`
      (`self.UpdateVisibility`))))

(event `OnRoundOverDelegate_Event_0`
  (params (RoundEndReason :type "ERoundConclusion Enum" :default "Generic") (WinningTeam :type Byte)))

(event `UpdateVisibility`
  (bind _discovered (`self.Discovered`))
  (bind _crate (`self.Crate`))
  (`SceneComponent.SetVisibility` (`self.StaticMesh`) (and (`self.Initialized`) (not _discovered)) false)
  (`SceneComponent.SetVisibility` (`self.StaticMesh2`) (and (`self.Initialized`) (not _discovered)) false)
  (if (`KismetSystemLibrary.IsValid` _crate)
    (if (not _discovered)
      (`self.K2_DestroyActor` _crate))))

(event `OnRoundActive`
  (bind _crate (`self.Crate`))
  (if (`KismetSystemLibrary.IsValid` _crate)
    (`self.K2_DestroyActor` _crate)
    (set `self.Discovered` false)
    (`self.UpdateVisibility`)))

(event `self.ReceiveActorBeginOverlap`
  (params (OtherActor :type "Actor Object Reference"))
  ;[1 1 1] Discovery
  (`/Engine/EditorBlueprintResources/ActorMacros.Switch Has Authority`
    (:`Authority`
      (if (`self.Initialized`)
        (if (`KismetMathLibrary.ClassIsChildOf` (`GameplayStatics.GetObjectClass` OtherActor) "/Script/Insurgency.INSSoldier")
          (bind _asbp_character_player (cast `/Game/Game/Actors/Characters/BP_Character_Player` OtherActor))
          (if (== (`INSSoldier.TeamId` _asbp_character_player) (`self.DefendingTeam`))
            (if (not (`KismetArrayLibrary.Array_Contains` (`self.PlayersInside`) _asbp_character_player))
              (`self.PlayerOverlap` _asbp_character_player)
              (`self.PlayerOverlap_Event` _asbp_character_player)
              (`KismetArrayLibrary.Array_AddUnique` (`self.PlayersInside`) _asbp_character_player))))))))

(event `self.ReceiveActorEndOverlap`
  (params (OtherActor :type "Actor Object Reference"))
  ;[1 1 1] Discovery
  (`/Engine/EditorBlueprintResources/ActorMacros.Switch Has Authority`
    (:`Authority`
      (if (`self.Initialized`)
        (if (`KismetMathLibrary.ClassIsChildOf` (`GameplayStatics.GetObjectClass` OtherActor) "/Script/Insurgency.INSSoldier")
          (bind _asbp_character_player (cast `/Game/Game/Actors/Characters/BP_Character_Player` OtherActor))
          (if (`KismetArrayLibrary.Array_Contains` (`self.PlayersInside`) _asbp_character_player)
            (if (not (`self.IsOverlappingActor` _asbp_character_player self))
              (`KismetArrayLibrary.Array_RemoveItem` (`self.PlayersInside`) _asbp_character_player))))))))

(event `PlayerOverlap_Event`
  (params (Soldier :type "INSSoldier Object Reference"))
  (if (not (`self.Discovered`))
    (set `self.Discovered` true)
    (if (`self.AlwaysActive`)
      (bind _returnvalue (`|SpawnActorFromClass` "/Game/Game/Actors/World/BP_SupplyCrate_Base.BP_SupplyCrate_Base_C" (`self.GetTransform`) "AlwaysSpawn" "OverrideRootScale" null null))
      (set `self.Crate` _returnvalue)
      (else
        (bind _returnvalue_2 (`|SpawnActorFromClass` "/CustomScenario/Blueprints/Operation/BP_SupplyCrate_OperationLimited.BP_SupplyCrate_OperationLimited_C" (`self.GetTransform`) "AlwaysSpawn" "OverrideRootScale" null null))
        (set `self.Crate` _returnvalue_2)))))

(fn `AutoSize`
  (locals (NewVar_0 :type "Vector Structure") (AutoSizerTraces :type "Array of Vector Structure"))
  (bind _autosizertraces (`local.AutoSizerTraces`))
  (bind _box (`self.Box`))
  (bind _newvar_0 (`local.NewVar_0`))
  (bind _box_2 (`self.Box`))
  (bind _autosizer (`self.AutoSizer`))
  (bind _returnvalue (`SceneComponent.K2_GetComponentLocation` _autosizer))
  (bind _output (`|GetArrayItem` _autosizertraces 5))
  (bind _output_2 (`|GetArrayItem` _autosizertraces 4))
  (bind _output_3 (`|GetArrayItem` _autosizertraces))
  (bind _output_4 (`|GetArrayItem` _autosizertraces 1))
  (bind _output_5 (`|GetArrayItem` _autosizertraces 2))
  (bind _output_6 (`|GetArrayItem` _autosizertraces 3))
  (bind _returnvalue_2 (`KismetMathLibrary.Normal` (`SceneComponent.GetUpVector` _autosizer)))
  (bind _returnvalue_3 (`KismetMathLibrary.Normal` (`SceneComponent.GetForwardVector` _autosizer)))
  (bind _returnvalue_4 (`KismetMathLibrary.Normal` (`SceneComponent.GetRightVector` _autosizer)))
  (bind _returnvalue_5 (+ _returnvalue (* _returnvalue_3 -200.0)))
  (bind _returnvalue_6 (+ _returnvalue (* _returnvalue_3 200.0)))
  (bind _returnvalue_7 (+ _returnvalue (* _returnvalue_4 200.0)))
  (bind _returnvalue_8 (+ _returnvalue (* _returnvalue_2 200.0)))
  (bind _returnvalue_9 (+ _returnvalue (* _returnvalue_2 -200.0)))
  (bind _returnvalue_10 (+ _returnvalue (* _returnvalue_4 -300.0)))
  (set `local.NewVar_0` _returnvalue)
  (set `local.AutoSizerTraces` (`|MakeArray` _returnvalue_6 _returnvalue_5 _returnvalue_7 _returnvalue_10 _returnvalue_8 _returnvalue_9))
  (`|ExecutionSequence`
    (:`then_0`
      (bind (_outhit _returnvalue_11) (`KismetSystemLibrary.LineTraceSingleByProfile` :`Start` _returnvalue :`End` _returnvalue_6 :`ProfileName` "Pawn" :`DrawDebugType` "ForDuration" :`TraceHitColor` (struct :`A` 1.0)))
      (if _returnvalue_11
        (`KismetArrayLibrary.Array_Set` (`local.AutoSizerTraces`) 0 (`.Location` (`GameplayStatics.BreakHitResult` _outhit))))
      (bind (_outhit_2 _returnvalue_12) (`KismetSystemLibrary.LineTraceSingleByProfile` :`Start` _returnvalue :`End` _returnvalue_5 :`ProfileName` "Pawn" :`DrawDebugType` "ForDuration" :`TraceColor` (struct :`R` 0.182292 :`A` 1.0) :`TraceHitColor` (struct :`A` 1.0)))
      (if _returnvalue_12
        (`KismetArrayLibrary.Array_Set` (`local.AutoSizerTraces`) 1 (`.Location` (`GameplayStatics.BreakHitResult` _outhit_2)))))
    (:`then_1`
      (bind (_outhit_3 _returnvalue_13) (`KismetSystemLibrary.LineTraceSingleByProfile` :`Start` _returnvalue :`End` _returnvalue_7 :`ProfileName` "Pawn" :`DrawDebugType` "ForDuration" :`TraceColor` (struct :`G` 1.0 :`A` 1.0) :`TraceHitColor` (struct :`A` 1.0)))
      (if _returnvalue_13
        (`KismetArrayLibrary.Array_Set` (`local.AutoSizerTraces`) 2 (`.Location` (`GameplayStatics.BreakHitResult` _outhit_3))))
      (bind (_outhit_4 _returnvalue_14) (`KismetSystemLibrary.LineTraceSingleByProfile` :`Start` _returnvalue :`End` _returnvalue_10 :`ProfileName` "Pawn" :`DrawDebugType` "ForDuration" :`TraceColor` (struct :`G` 0.333333 :`A` 1.0) :`TraceHitColor` (struct :`A` 1.0)))
      (if _returnvalue_14
        (`KismetArrayLibrary.Array_Set` (`local.AutoSizerTraces`) 3 (`.Location` (`GameplayStatics.BreakHitResult` _outhit_4)))))
    (:`then_2`
      (bind (_outhit_5 _returnvalue_15) (`KismetSystemLibrary.LineTraceSingleByProfile` :`Start` _returnvalue :`End` _returnvalue_8 :`ProfileName` "Pawn" :`DrawDebugType` "ForDuration" :`TraceColor` (struct :`B` 1.0 :`A` 1.0) :`TraceHitColor` (struct :`A` 1.0)))
      (if _returnvalue_15
        (`KismetArrayLibrary.Array_Set` (`local.AutoSizerTraces`) 4 (`.Location` (`GameplayStatics.BreakHitResult` _outhit_5))))
      (bind (_outhit_6 _returnvalue_16) (`KismetSystemLibrary.LineTraceSingleByProfile` :`Start` _returnvalue :`End` _returnvalue_9 :`ProfileName` "Pawn" :`DrawDebugType` "ForDuration" :`TraceColor` (struct :`B` 0.359375 :`A` 1.0) :`TraceHitColor` (struct :`A` 1.0)))
      (if _returnvalue_16
        (`KismetArrayLibrary.Array_Set` (`local.AutoSizerTraces`) 5 (`.Location` (`GameplayStatics.BreakHitResult` _outhit_6)))))
    (:`then_3`
      (`SceneComponent.K2_SetRelativeLocation` _box_2 (`SceneComponent.RelativeLocation` (`self.AutoSizer`)) false false)
      (`SceneComponent.K2_AddWorldOffset` _box_2 (+ (- (`KismetMathLibrary.VLerp` _output_3 _output_4 0.5) _newvar_0) (- (`KismetMathLibrary.VLerp` _output_5 _output_6 0.5) _newvar_0) (- (`KismetMathLibrary.VLerp` _output_2 _output 0.5) _newvar_0)) false false)
      (`SceneComponent.K2_SetRelativeRotation` _box (`SceneComponent.RelativeRotation` (`self.AutoSizer`)) false false)
      (`SceneComponent.SetRelativeScale3D` _box (1.0 1.0 1.0))
      (`BoxComponent.SetBoxExtent` _box (* (`KismetMathLibrary.MakeVector` (`KismetMathLibrary.Vector_Distance` _output_3 _output_4) (`KismetMathLibrary.Vector_Distance` _output_5 _output_6) (`KismetMathLibrary.Vector_Distance` _output_2 _output)) 0.5) true)
      (return))))

(fn `OnRep_AlwaysActive`)

(fn `OnRep_Discovered`
  (`self.UpdateVisibility`)
  (return))

(fn `OnRep_Initialized`
  (`self.UpdateVisibility`)
  (return))

(fn `UserConstructionScript`)