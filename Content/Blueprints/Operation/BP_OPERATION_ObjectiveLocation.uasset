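; Operation mode objective location that, when marked real, spawns a team-specific weapon cache or a drainable GAZ fuel tanker, per ObjectiveType.
; The server tracks defending players inside the box and reports their entry.
; Destroying or draining the objective deactivates it, advances its stage and marks it discovered, with OnRep functions relaying state to event dispatchers.
; An editor AutoSize event fits the box to surroundings using six axis line traces.
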(event `AutoSize`
  ;[0 0.7489 1] Editor AutoSizer
  (`self.FuncAutoSize`))

(event `self.ReceiveBeginPlay`
  ;[1 1 1] BeginPlay
  (`/Engine/EditorBlueprintResources/ActorMacros.Switch Has Authority`
    (:`Authority`
      (`KismetSystemLibrary.Delay` 1.0)
      (bind _askwioperation_gamemode (cast `/CustomScenario/Blueprints/Operation/KWIOperationGamemode` (`GameplayStatics.GetGameMode`))
        (:`then`
          (set `self.DefendingTeam` (`INSGameMode.GetDefendingTeam` _askwioperation_gamemode))
          (set `self.AttackingTeam` (`INSGameMode.GetAttackingTeam` _askwioperation_gamemode))
          (`|ExecutionSequence`
            (:`then_0`
              (if (`self.Real`)
                (`self.RealStateChanged_Event` null)))))
        (:`CastFailed`
          (`KismetSystemLibrary.K2_SetTimerDelegate` (delegate `JustInCase`) 1.0))))))

(event `JustInCase`
  ;[1 1 1] BeginPlay
)

(event `self.ReceiveActorBeginOverlap`
  (params (OtherActor :type "Actor Object Reference"))
  ;[1 1 1] Discovery
  (`/Engine/EditorBlueprintResources/ActorMacros.Switch Has Authority`
    (:`Authority`
      (if (`self.Initialized`)
        (if (`KismetMathLibrary.ClassIsChildOf` (`GameplayStatics.GetObjectClass` OtherActor) "/Script/Insurgency.INSSoldier")
          (bind _asbp_character_player (cast `/Game/Game/Actors/Characters/BP_Character_Player` OtherActor))
          (if (== (`INSSoldier.TeamId` _asbp_character_player) (`self.DefendingTeam`))
            (if (not (`KismetArrayLibrary.Array_Contains` (`self.PlayersInside`) _asbp_character_player))
              (`self.PlayerOverlap` self _asbp_character_player)
              (`KismetArrayLibrary.Array_AddUnique` (`self.PlayersInside`) _asbp_character_player))))))))

(event `PostAudio`
  (params (`AK Audio Event` :type "AkAudioEvent Object Reference") (LocationOffset :type "Vector Structure"))
  (bind _insaudio (`self.INSAudio`))
  ;[1 1 1] AudioEvent
  (set `AkGameObject.AkAudioEvent` `AK Audio Event` _insaudio)
  (`SceneComponent.K2_SetRelativeLocation` _insaudio LocationOffset false false)
  (`AkGameObject.PostAssociatedAkEvent` :`self` _insaudio :`PostEventCallback` (delegate `OnAKEnd`)))

(event `self.ReceiveActorEndOverlap`
  (params (OtherActor :type "Actor Object Reference"))
  ;[1 1 1] Discovery
  (`/Engine/EditorBlueprintResources/ActorMacros.Switch Has Authority`
    (:`Authority`
      (if (`self.Initialized`)
        (if (`KismetMathLibrary.ClassIsChildOf` (`GameplayStatics.GetObjectClass` OtherActor) "/Script/Insurgency.INSSoldier")
          (bind _asbp_character_player (cast `/Game/Game/Actors/Characters/BP_Character_Player` OtherActor))
          (if (`KismetArrayLibrary.Array_Contains` (`self.PlayersInside`) _asbp_character_player)
            (if (not (`self.IsOverlappingActor` _asbp_character_player self))
              (`KismetArrayLibrary.Array_RemoveItem` (`self.PlayersInside`) _asbp_character_player))))))))

(event `OnAKEnd`
  (params (CallbackType :type "EAkCallbackType Enum" :default "EndOfEvent") (CallbackInfo :type "AkCallbackInfo Object Reference"))
  ;[1 1 1] AudioEvent
)

(event `RealStateChanged_Event`
  (params (ObjectiveLocation :type "/Game/Blueprints/Operation/BP_OPERATION_ObjectiveLocation Object Reference") (`New Real` :type Boolean))
  ;[1 1 1] Real State
  (`/Engine/EditorBlueprintResources/ActorMacros.Switch Has Authority`
    (:`Authority`
      (if (`self.Real`)
        (`self.ProxySetup`)
        (else
          (`self.ProxyCleanup`))))))

(event `ProxySetup`
  (bind _returnvalue (`self.GetTransform`))
  (bind _proxydestructible (`self.ProxyDestructible`))
  (bind _usableactor (`self.UsableActor`))
  ;[1 1 1] Proxy
  (if (not (`self.ProxyDeployed`))
    (set `self.ProxyDeployed` true)
    (switch `int` (`KismetMathLibrary.Conv_ByteToInt` (`self.Objective Type`))
      (:`Default`
        ;[1 1 1] Cache setup
        (bind _returnvalue_2 (`|SpawnActorFromClass` (select `byte` (`self.DefendingTeam`) :`0` "/Game/Game/Actors/Objectives/Obj_WeaponCache_Ins.Obj_WeaponCache_Ins_C" :`1` "/Game/Game/Actors/Objectives/Obj_WeaponCache_Sec.Obj_WeaponCache_Sec_C" :!type "Actor Class Reference") (`self.GetTransform`) "AlwaysSpawn" "OverrideRootScale" null null :!label _label))
        (bind _asobjective_destructible (cast `ObjectiveDestructible` _returnvalue_2))
        (set `self.ProxyDestructible` _asobjective_destructible)
        (if (`KismetSystemLibrary.IsValid` _proxydestructible)
          (add `ObjectiveDestructible.OnDestructibleObjectiveStateChangedDelegate` _proxydestructible (`|CreateDelegate` :!event `OnCacheBlownUp`))
          (set `self.ObjectiveStage` 0)
          (set `self.ObjectiveActive` true)))
      (:`0`
        (goto _label))
      (:`1`
        (bind _returnvalue_3 (`|SpawnActorFromClass` "/CustomScenario/Blueprints/Operation/Operation_Obj_Vehicle_Gaz.Operation_Obj_Vehicle_Gaz_C" _returnvalue "AlwaysSpawn" "OverrideRootScale" null null))
        (bind _returnvalue_4 (`|SpawnActorFromClass` "/CustomScenario/Blueprints/Operation/Buttons/BP_SimpleUsable_Fuel.BP_SimpleUsable_Fuel_C" _returnvalue "AlwaysSpawn" "OverrideRootScale" null null))
        (bind _output_get (set `self.UsableActor` _returnvalue_4))
        (set `/CustomScenario/Blueprints/Operation/Buttons/BP_SimpleUsable.Offset` (`KismetMathLibrary.MakeTransform` (-90.0 0.0 100.0) (struct) (10.0 12.0 5.0)) _output_get)
        (set `/CustomScenario/Blueprints/Operation/Buttons/BP_SimpleUsable.Parent` _returnvalue_3 _output_get)
        (add `ObjectiveDestructible.OnDestructibleObjectiveStateChangedDelegate` _returnvalue_3 (`|CreateDelegate` :!event `OnCacheBlownUp`))
        (add `/CustomScenario/Blueprints/Operation/Buttons/BP_SimpleUsable.OnUseCompleteDispatch` _usableactor (delegate `OnDrained`))
        (add `/CustomScenario/Blueprints/Operation/Buttons/BP_SimpleUsable.OnUseDispatch` _usableactor (delegate `OnStartDrain`))
        (set `self.ObjectiveStage` 0)
        (set `self.ObjectiveActive` true)))))

(event `OnCacheBlownUp`
  (params (Objective :type "ObjectiveDestructible Object Reference") (NewState :type "EDestructibleObjectiveState Enum" :default "Normal"))
  ;[1 1 1] On real cache destruction
  (if (and (`|EnumEquality` NewState "Destroyed") (`self.ObjectiveActive`))
    (set `self.ObjectiveStage` 1)
    (set `self.ObjectiveActive` false)
    (set `self.Discovered` true)))

(event `OnDrained`
  (params (Actor :type "Actor Object Reference") (Pawn :type "INSSoldier Object Reference"))
  (bind _usableactor (`self.UsableActor`))
  (if (`self.ObjectiveActive`)
    (set `self.ObjectiveStage` 1)
    (set `self.ObjectiveActive` false)
    (set `self.Discovered` true)
    (`self.PostAudio` "/Game/Audio/wwise/Sandstorm/Physics/Dynamic_Props/Objectives/FuelTanker/Play_FuelTanker_Disabled.Play_FuelTanker_Disabled" (-200.0 0.0 180.0))
    (clear `/CustomScenario/Blueprints/Operation/Buttons/BP_SimpleUsable.OnUseDispatch` _usableactor)
    (clear `/CustomScenario/Blueprints/Operation/Buttons/BP_SimpleUsable.OnUseCompleteDispatch` _usableactor)
    (set `/CustomScenario/Blueprints/Operation/Buttons/BP_SimpleUsable.EnabledUsable` false _usableactor)))

(event `OnStartDrain`
  (params (Actor :type "Actor Object Reference") (Pawn :type "INSSoldier Object Reference"))
  (`/Engine/EditorBlueprintResources/StandardMacros.DoOnce` false :!label _label_2
    (:`Completed`
      (`self.PostAudio` "/Game/Audio/wwise/Sandstorm/Physics/Dynamic_Props/Objectives/FuelTanker/Play_FuelTanker_Rigging.Play_FuelTanker_Rigging" (-90.0 0.0 100.0))
      (`KismetSystemLibrary.Delay` 2.0)
      (goto _label_2 :!via `Reset`))))

(event `ProxyCleanup`
  (bind _proxydestructible (`self.ProxyDestructible`))
  (bind _usableactor (`self.UsableActor`))
  ;[1 1 1] ProxyClean
  (set `self.ProxyDeployed` false)
  (switch `int` (`KismetMathLibrary.Conv_ByteToInt` (`self.Objective Type`))
    (:`Default`
      _)
    (:`0`
      _)
    (:`1`
      _))
  (if (`KismetSystemLibrary.IsValid` _proxydestructible)
    (clear `ObjectiveDestructible.OnDestructibleObjectiveStateChangedDelegate` _proxydestructible)
    (`self.K2_DestroyActor` _proxydestructible)
    (set `self.ProxyDestructible` null))
  (if (== (`self.Objective Type`) 1)
    (if (`KismetSystemLibrary.IsValid` _usableactor)
      (clear `/CustomScenario/Blueprints/Operation/Buttons/BP_SimpleUsable.OnUseDispatch` _usableactor)
      (clear `/CustomScenario/Blueprints/Operation/Buttons/BP_SimpleUsable.OnUseCompleteDispatch` _usableactor)
      (`self.K2_DestroyActor` _usableactor))))

(event `StageStateChanged_Event`
  (params (ObjectiveLocation :type "/Game/Blueprints/Operation/BP_OPERATION_ObjectiveLocation Object Reference") (`New Stage` :type Byte))
  (`/Engine/EditorBlueprintResources/ActorMacros.Switch Has Authority`
    (:`Authority`
      (if (> `New Stage` 0)
        (set `self.Discovered` true)))))

(fn `FuncAutoSize`
  (bind _autosizertraces (`self.AutoSizerTraces`))
  (bind _box (`self.Box`))
  (bind _autosizer (`self.AutoSizer`))
  (bind _newvar_0 (`self.NewVar_0`))
  (bind _box_2 (`self.Box`))
  (bind _returnvalue (`SceneComponent.K2_GetComponentLocation` _autosizer))
  (bind _output (`|GetArrayItem` _autosizertraces 5))
  (bind _output_2 (`|GetArrayItem` _autosizertraces 4))
  (bind _output_3 (`|GetArrayItem` _autosizertraces))
  (bind _output_4 (`|GetArrayItem` _autosizertraces 1))
  (bind _output_5 (`|GetArrayItem` _autosizertraces 2))
  (bind _output_6 (`|GetArrayItem` _autosizertraces 3))
  (bind _returnvalue_2 (`KismetMathLibrary.Normal` (`SceneComponent.GetUpVector` _autosizer)))
  (bind _returnvalue_3 (`KismetMathLibrary.Normal` (`SceneComponent.GetForwardVector` _autosizer)))
  (bind _returnvalue_4 (`KismetMathLibrary.Normal` (`SceneComponent.GetRightVector` _autosizer)))
  (bind _returnvalue_5 (+ _returnvalue (* _returnvalue_3 -1000.0)))
  (bind _returnvalue_6 (+ _returnvalue (* _returnvalue_3 1000.0)))
  (bind _returnvalue_7 (+ _returnvalue (* _returnvalue_4 1000.0)))
  (bind _returnvalue_8 (+ _returnvalue (* _returnvalue_2 300.0)))
  (bind _returnvalue_9 (+ _returnvalue (* _returnvalue_2 -1000.0)))
  (bind _returnvalue_10 (+ _returnvalue (* _returnvalue_4 -1000.0)))
  (set `self.NewVar_0` _returnvalue)
  (set `self.AutoSizerTraces` (`|MakeArray` _returnvalue_6 _returnvalue_5 _returnvalue_7 _returnvalue_10 _returnvalue_8 _returnvalue_9))
  (`|ExecutionSequence`
    (:`then_0`
      (bind (_outhit _returnvalue_11) (`KismetSystemLibrary.LineTraceSingleByProfile` :`Start` _returnvalue :`End` _returnvalue_6 :`ProfileName` "Pawn" :`DrawDebugType` "ForDuration" :`TraceHitColor` (struct :`A` 1.0)))
      (if _returnvalue_11
        (`KismetArrayLibrary.Array_Set` (`self.AutoSizerTraces`) 0 (`.Location` (`GameplayStatics.BreakHitResult` _outhit))))
      (bind (_outhit_2 _returnvalue_12) (`KismetSystemLibrary.LineTraceSingleByProfile` :`Start` _returnvalue :`End` _returnvalue_5 :`ProfileName` "Pawn" :`DrawDebugType` "ForDuration" :`TraceColor` (struct :`R` 0.182292 :`A` 1.0) :`TraceHitColor` (struct :`A` 1.0)))
      (if _returnvalue_12
        (`KismetArrayLibrary.Array_Set` (`self.AutoSizerTraces`) 1 (`.Location` (`GameplayStatics.BreakHitResult` _outhit_2)))))
    (:`then_1`
      (bind (_outhit_3 _returnvalue_13) (`KismetSystemLibrary.LineTraceSingleByProfile` :`Start` _returnvalue :`End` _returnvalue_7 :`ProfileName` "Pawn" :`DrawDebugType` "ForDuration" :`TraceColor` (struct :`G` 1.0 :`A` 1.0) :`TraceHitColor` (struct :`A` 1.0)))
      (if _returnvalue_13
        (`KismetArrayLibrary.Array_Set` (`self.AutoSizerTraces`) 2 (`.Location` (`GameplayStatics.BreakHitResult` _outhit_3))))
      (bind (_outhit_4 _returnvalue_14) (`KismetSystemLibrary.LineTraceSingleByProfile` :`Start` _returnvalue :`End` _returnvalue_10 :`ProfileName` "Pawn" :`DrawDebugType` "ForDuration" :`TraceColor` (struct :`G` 0.333333 :`A` 1.0) :`TraceHitColor` (struct :`A` 1.0)))
      (if _returnvalue_14
        (`KismetArrayLibrary.Array_Set` (`self.AutoSizerTraces`) 3 (`.Location` (`GameplayStatics.BreakHitResult` _outhit_4)))))
    (:`then_2`
      (bind (_outhit_5 _returnvalue_15) (`KismetSystemLibrary.LineTraceSingleByProfile` :`Start` _returnvalue :`End` _returnvalue_8 :`ProfileName` "Pawn" :`DrawDebugType` "ForDuration" :`TraceColor` (struct :`B` 1.0 :`A` 1.0) :`TraceHitColor` (struct :`A` 1.0)))
      (if _returnvalue_15
        (`KismetArrayLibrary.Array_Set` (`self.AutoSizerTraces`) 4 (`.Location` (`GameplayStatics.BreakHitResult` _outhit_5))))
      (bind (_outhit_6 _returnvalue_16) (`KismetSystemLibrary.LineTraceSingleByProfile` :`Start` _returnvalue :`End` _returnvalue_9 :`ProfileName` "Pawn" :`DrawDebugType` "ForDuration" :`TraceColor` (struct :`B` 0.359375 :`A` 1.0) :`TraceHitColor` (struct :`A` 1.0)))
      (if _returnvalue_16
        (`KismetArrayLibrary.Array_Set` (`self.AutoSizerTraces`) 5 (`.Location` (`GameplayStatics.BreakHitResult` _outhit_6)))))
    (:`then_3`
      (`SceneComponent.K2_SetRelativeLocation` _box_2 (`SceneComponent.RelativeLocation` (`self.AutoSizer`)) false false)
      (`SceneComponent.K2_AddWorldOffset` _box_2 (+ (- (`KismetMathLibrary.VLerp` _output_3 _output_4 0.5) _newvar_0) (- (`KismetMathLibrary.VLerp` _output_5 _output_6 0.5) _newvar_0) (- (`KismetMathLibrary.VLerp` _output_2 _output 0.5) _newvar_0)) false false)
      (`SceneComponent.K2_SetRelativeRotation` _box (`SceneComponent.RelativeRotation` (`self.AutoSizer`)) false false)
      (`SceneComponent.SetRelativeScale3D` _box (1.0 1.0 1.0))
      (`BoxComponent.SetBoxExtent` _box (* (`KismetMathLibrary.MakeVector` (`KismetMathLibrary.Vector_Distance` _output_3 _output_4) (`KismetMathLibrary.Vector_Distance` _output_5 _output_6) (`KismetMathLibrary.Vector_Distance` _output_2 _output)) 0.5) true)
      (return))))

(fn `OnRep_Discovered`
  (`self.DiscoveredStateChanged` self (`self.Discovered`))
  (return))

(fn `OnRep_Initialized`
  (`self.InitilizedStateChanged` self (`self.Initialized`))
  (return))

(fn `OnRep_ObjectiveActive`
  (`self.ActiveStateChanged` self (`self.ObjectiveActive`))
  (return))

(fn `OnRep_ObjectiveStage`
  (`self.StageStateChanged` self (`self.ObjectiveStage`))
  (return))

(fn `OnRep_Real`
  (`self.RealStateChanged` self (`self.Real`))
  (return))

(fn `UserConstructionScript`
  (`AddComponent|NODE_AddStaticMeshComponent-0`)
  (`BillboardComponent.SetSprite` (`self.Type`) (select `byte` (`self.Objective Type`) :`0` "/Game/UI/Textures/T_UI_Icon_RigginExplosives.T_UI_Icon_RigginExplosives" :`1` "/Game/UI/Textures/InGame/T_UI_Obj_Fuel.T_UI_Obj_Fuel" :`2` "/Game/UI/Textures/InGame/T_UI_Obj_Assassinate_Beret.T_UI_Obj_Assassinate_Beret" :`3` "/Game/UI/Textures/InGame/T_UI_Obj_Assassinate_Cap.T_UI_Obj_Assassinate_Cap" :`4` "/Game/UI/Textures/InGame/T_UI_Obj_Character.T_UI_Obj_Character" :`5` "/Game/UI/Textures/InGame/T_UI_Obj_Regroup.T_UI_Obj_Regroup" :!type "Texture2D Object Reference"))
  (switch `int` (`KismetMathLibrary.Conv_ByteToInt` (`self.Objective Type`))
    (:`Default`
      (`SceneComponent.SetVisibility` (`self.StaticMesh`) false false))
    (:`1`
      (`StaticMeshComponent.SetStaticMesh` (`self.StaticMesh`) "/Game/Environment/Props/Vehicles/SM_VHC_GAZTanker.SM_VHC_GAZTanker"))))