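; BP_SupplyCrate_OperationLimited is a limited-use supply crate that visually shows how many uses remain through instanced ammo box meshes.
; When the uses-left count updates, it removes the mesh instance at the new count's index and reveals a decal once none remain.
; When the count equals the allowed maximum, as on round reset, it rebuilds all instances from stored transforms and hides the decal.
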(event `self.BlueprintOnUsesLeftUpdated`
  (bind _usesleft (`self.UsesLeft`))
  (bind _ammomeshes (`self.AmmoMeshes`))
  (bind _decal (`self.Decal`))
  (if (== (`self.TimesAllowedToBeUsed`) _usesleft)
    ;[1 1 1] This resets the Ammo Box Meshes on Round Reset
    (`InstancedStaticMeshComponent.ClearInstances` _ammomeshes)
    (for _index (range (`self.TimesAllowedToBeUsed`))
      (`InstancedStaticMeshComponent.AddInstance` _ammomeshes (`|GetArrayItem` (`self.AmmoMeshesTransforms`) _index)))
    (`SceneComponent.SetVisibility` _decal false false)
    (else
      (`InstancedStaticMeshComponent.RemoveInstance` _ammomeshes _usesleft)
      (if (== (`self.UsesLeft`) 0)
        (`SceneComponent.SetVisibility` _decal true false)))))

(fn `UserConstructionScript`)