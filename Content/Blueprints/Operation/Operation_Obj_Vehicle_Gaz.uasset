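; Destructible operation objective Blueprint for a Gaz vehicle that plays effects when destroyed.
; The destruction effects event activates the BoomParticle system and posts the Audio component's associated Wwise event.
; One second after BeginPlay it binds to the objective's state change delegate and prints each new state as a string.
; An unconnected check for live rigged explosives never runs, and the construction script is empty.
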(event `self.ReceiveBeginPlay`
  (`KismetSystemLibrary.Delay` 1.0)
  (add `self.OnDestructibleObjectiveStateChangedDelegate` (delegate `CustomEvent_0`)))

(event `CustomEvent_0` :!signature `self.OnDestructibleObjectiveStateChangedDelegate`
  (params (Objective :type "ObjectiveDestructible Object Reference") (NewState :type "EDestructibleObjectiveState Enum" :default "Normal"))
  (`KismetSystemLibrary.PrintString` (`|GetEnumeratorNameAsString` NewState)))

(event `self.OnPlayDestructionEffects`
  (`ActorComponent.Activate` (`self.BoomParticle`) false)
  (`AkComponent.PostAssociatedAkEvent` :`self` (`self.Audio`)))

(fn `UserConstructionScript`)