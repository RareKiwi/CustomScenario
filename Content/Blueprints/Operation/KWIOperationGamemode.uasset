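; Operation co-op gamemode that adds optional hardcore HUD and respawn rules.
; On server BeginPlay it spawns its manager actor and optional bot mover, and can swap in the hardcore HUD.
; With hardcore respawn, defending-team players spawning outside wave one or a final-wave counterattack are stripped to pistol, melee and binocular weapons plus a fallback primary.
; Their saved loadout is restored afterwards; other spawns use normal inventory.
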(event `self.ReceiveBeginPlay`
  (`/Engine/EditorBlueprintResources/ActorMacros.Switch Has Authority`
    (:`Authority`
      (`/Engine/EditorBlueprintResources/StandardMacros.DoOnce` false
        (:`Completed`
          (`|ExecutionSequence`
            (:`then_0`
              (bind _returnvalue (`|SpawnActorFromClass` "/CustomScenario/Blueprints/Operation/BP_KWIOperationGamemode_Manager.BP_KWIOperationGamemode_Manager_C" (`KismetMathLibrary.MakeTransform` (0.0 0.0 0.0)) "AlwaysSpawn" "OverrideRootScale" null null))
              (set `self.GamemodeManager` _returnvalue)
              (if (`self.BotMover`)
                (`|SpawnActorFromClass` "/CustomScenario/Blueprints/Operation/BP_BotMover.BP_BotMover_C" (`KismetMathLibrary.MakeTransform` (0.0 0.0 0.0)) "AlwaysSpawn" "OverrideRootScale" null null)))
            (:`then_1`
              (if (`self.HardcoreHUD`)
                (set `self.HUDClass` "/CustomScenario/Blueprints/Operation/BP_HUD_CoopOperationHardcore.BP_HUD_CoopOperationHardcore_C")))))))))

(event `self.GiveSoldierInventory`
  (params (Player :type "INSSoldier Object Reference") (bFromResupply :type Boolean))
  (`KismetSystemLibrary.PrintString` "Hello")
  (if (`self.HardcoreRespawn`)
    (if (== (`INSSoldier.TeamId` Player) (`self.GetDefendingTeam`))
      (if (== (`self.CurrentWave`) 1)
        (`parent.GiveSoldierInventory` Player bFromResupply :!label _label)
        (else
          (if (`self.IsFinalWave`)
            (if (`ObjectiveBase.bCounterAttack` (`self.GetFirstActiveObjective`))
              (goto _label)
              (else
                _)))
          (bind _asinsplayer_controller (cast `INSPlayerController` (`Pawn.GetController` Player))
            (:`then`
              (bind _inventorycomponent (`INSPlayerController.InventoryComponent` _asinsplayer_controller))
              (bind _outloadout (`PlayerInventoryComponent.GetLoadout` _inventorycomponent true))
              (set `self.StoreLoadout` _outloadout)
              (bind (_arrayindex _arrayelement) (`/Engine/EditorBlueprintResources/StandardMacros.ReverseForEachLoop` _outloadout)
                (:`LoopBody`
                  (bind _output (`|ConvertAsset` (`.Item` (break `BasicLoadoutItem` _arrayelement))))
                  (`KismetSystemLibrary.PrintString` (`KismetTextLibrary.Conv_TextToString` (defaults `Object` _output)))
                  (bind _asitem_weapon (castclass `ItemWeapon` _output))
                  (castclass `/Game/Game/Actors/Weapons/SideArm/BP_Firearm_PistolBase` _asitem_weapon
                    (:`CastFailed`
                      (castclass `/Game/Game/Actors/Weapons/Melee/BP_Melee` _asitem_weapon
                        (:`CastFailed`
                          (castclass `ItemBinocular` _asitem_weapon
                            (:`CastFailed`
                              (`InventoryComponent.RemoveItem` _inventorycomponent _arrayindex))))))))
                (:`Completed`
                  (`PlayerInventoryComponent.GiveInventoryItems` _inventorycomponent)
                  (`InventoryComponent.CheckFallbackFor` _inventorycomponent Player (`|MakeMap` "Primary" (`self.FallbackPrimary`) :!type "EItemSlot Enum"))
                  (`INSSoldier.EquipInventoryItem` Player (`INSSoldier.GetEquipableInSlot` Player "Primary") true)
                  (`PlayerInventoryComponent.SetLoadout` _inventorycomponent (`self.StoreLoadout`)))))
            (:`CastFailed`
              (goto _label)))))
      (else
        (goto _label)))
    (else
      (goto _label))))

(fn `UserConstructionScript`)