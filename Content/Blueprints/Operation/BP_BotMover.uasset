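; Server-side helper for Survival mode that makes living defending-team AI bots follow the first player in a chain.
; Once a round goes active, a looping timer drives the follow pass, each bot trailing the one before it with distance-based walk, run or sprint.
; Wandering or chasing behaviours are overridden with priority moves and melee weapons dropped for guns, while grenade reactions and combat cover are left alone.
; Unpackaged builds give these bots god mode.
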(event `CustomEvent_0`
  (`/Engine/EditorBlueprintResources/StandardMacros.DoOnce` false
    (:`Completed`
      (`KismetSystemLibrary.K2_SetTimerDelegate` (`|CreateDelegate` :!event `BotMover`) 0.2 true)
      (remove `INSMultiplayerMode.OnRoundActiveDelegate` (`self.Gamemode`) (`|CreateDelegate` :!event `CustomEvent_0`)))))

(event `self.ReceiveBeginPlay`
  (`/Engine/EditorBlueprintResources/ActorMacros.Switch Has Authority`
    (:`Authority`
      (`KismetSystemLibrary.Delay` 1.0)
      (bind _asinssurvival_game_mode (cast `INSSurvivalGameMode` (`GameplayStatics.GetGameMode`)))
      (bind _output_get (set `self.Gamemode` _asinssurvival_game_mode))
      (add `INSMultiplayerMode.OnRoundActiveDelegate` _output_get (`|CreateDelegate` :!event `CustomEvent_0`)))))

(event `BotMover`
  (bind _returnvalue (`GameplayStatics.GetPlayerController` 0))
  (bind _friendbots (`self.FriendBots`))
  (bind _acceptradius (`self.acceptRadius`))
  (bind _returnvalue_2 (`Controller.K2_GetPawn` _returnvalue))
  ;[1 1 1] Bot mover
  (bind _outactors (`GameplayStatics.GetAllActorsOfClass` "/Script/Insurgency.INSAISoldierController"))
  (if (`KismetSystemLibrary.IsValid` _returnvalue)
    (if (`KismetSystemLibrary.IsValid` _returnvalue_2)
      (bind _asinssoldier (cast `INSSoldier` _returnvalue_2))
      (if (> (`INSCharacter.Health` _asinssoldier) 0.0)
        (`KismetArrayLibrary.Array_Clear` (`self.FriendBots`))
        (for _array_element _outactors
          (bind _returnvalue_3 (`INSAISoldierController.GetSoldier` _array_element))
          (if (`KismetSystemLibrary.IsValid` _returnvalue_3)
            (if (> (`INSCharacter.Health` _returnvalue_3) 0.0)
              (if (== (`INSAISoldierController.GetTeamId` _array_element) (`INSGameMode.GetDefendingTeam` (`self.Gamemode`)))
                (`KismetArrayLibrary.Array_Add` (`self.FriendBots`) _array_element)
                (if (not (`KismetSystemLibrary.IsPackagedForDistribution`))
                  (set `INSCharacter.bGodMode` true _returnvalue_3))))))
        (for (_array_element_2 _array_index) _friendbots
          (bind _returnvalue_4 (`BotBehaviorHandler.GetActiveBehavior` (`INSAISoldierController.GetBehaviorHandler` _array_element_2)))
          (if (`KismetSystemLibrary.IsValid` _returnvalue_4)
            (bind _returnvalue_5 (`BotBehavior.GetBehaviorName` _returnvalue_4))
            (bind _desiredmovereason (`INSAISoldierController.DesiredMoveReason` _array_element_2))
            (if (or (== _returnvalue_5 "Pursue") (== _returnvalue_5 "Flush Target") (== _returnvalue_5 "Investigate") (`KismetTextLibrary.EqualEqual_TextText` _desiredmovereason "Survival Fallback Wander") (== _returnvalue_5 "Retreat"))
              (bind _returnvalue_6 (`INSAISoldierController.GetSoldier` _array_element_2))
              (bind _currentweapon (`INSSoldier.CurrentWeapon` _returnvalue_6))
              (if (`KismetMathLibrary.ClassIsChildOf` (`GameplayStatics.GetObjectClass` _currentweapon) "/Game/Game/Actors/Weapons/Melee/BP_Melee.BP_Melee_C")
                (bind _asbp_melee (cast `/Game/Game/Actors/Weapons/Melee/BP_Melee` _currentweapon)
                  (:`then`
                    (`ItemBase.DropItem` _asbp_melee)
                    (bind _returnvalue_7 (`INSSoldier.GetItemInSlot` _returnvalue_6 "Primary"))
                    (if (`KismetSystemLibrary.IsValid` _returnvalue_7)
                      (bind _asitem_equipable (cast `ItemEquipable` _returnvalue_7)
                        (:`then`
                          (`INSSoldier.EquipInventoryItem` _returnvalue_6 _asitem_equipable false))
                        (:`CastFailed`
                          _))
                      (else
                        (bind _returnvalue_8 (`INSSoldier.GetItemInSlot` _returnvalue_6 "Secondary"))
                        (if (`KismetSystemLibrary.IsValid` _returnvalue_8)
                          (bind _asitem_equipable_2 (cast `ItemEquipable` _returnvalue_8)
                            (:`then`
                              (`INSSoldier.EquipInventoryItem` _returnvalue_6 _asitem_equipable_2 false))
                            (:`CastFailed`
                              _))))))
                  (:`CastFailed`
                    _)))
              (bind _returnvalue_9 (select `bool` (== _array_index 0) :`false` (`INSAISoldierController.GetSoldier` (`|GetArrayItem` _friendbots (`KismetMathLibrary.Clamp` (- _array_index 1) 0 (`KismetArrayLibrary.Array_LastIndex` _friendbots)))) :`true` _asinssoldier :!type "Actor Object Reference"))
              (bind _returnvalue_10 (`self.GetDistanceTo` _returnvalue_6 _returnvalue_9))
              (bind _returnvalue_11 (select `bool` (> _returnvalue_10 1600.0) :`false` (select `bool` (> _returnvalue_10 400.0) :`false` "Walk" :`true` "Run" :!type "EAIDesiredLocomotion Enum") :`true` "Sprint"))
              (`INSAISoldierController.MoveToActorSafe` _array_element_2 _returnvalue_9 "Move to Leader Force" _returnvalue_11 "Stand" "Important" true _acceptradius true)
              (elif (or (== _returnvalue_5 "Throw Grenade at Threat") (== _returnvalue_5 "FleeGrenade") (== _returnvalue_5 "Throw Back Grenade"))
                _
                (elif (not (and (== _returnvalue_5 "Attack Ranged") (`KismetTextLibrary.EqualEqual_TextText` _desiredmovereason "Taking Cover in Combat")))
                  (if (> _returnvalue_10 (+ (`self.acceptRadius`) (`self.deadzoneDistance`))) :!label _label
                    (`INSAISoldierController.MoveToActorSafe` _array_element_2 _returnvalue_9 "Move to Leader" _returnvalue_11 "Stand" "Low" true _acceptradius true)))))
            (else
              (goto _label))))))))

(fn `UserConstructionScript`)