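; UH-60 transport helicopter vehicle Blueprint that drives Wwise engine, rotor and turbine audio and handles engine failure from damage.
; Off dedicated servers, a one-second looping timer async-loads the sound bank, starts the three sounds once, and syncs seat audio.
; SyncSeatSound checks whether the local pawn is seated aboard, switching the turbine in/out RTPC and bus volumes.
; Engine part health at or below a quarter shuts the engine off once.
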(event `OnGearChanged`
  (`self.OnGearChange`))

(event `self.ReceiveBeginPlay`
  (if (not (`KismetSystemLibrary.IsDedicatedServer`))
    (`KismetSystemLibrary.K2_SetTimerDelegate` (delegate `CustomEvent_0`) 1.0 true)))

(event `CustomEvent_0`
  (`AkGameplayStatics.LoadBankAsync` "/Game/Audio/wwise/WwiseBanks/Vehicles/Air/Vehicle_UH60.Vehicle_UH60" (delegate `CustomEvent_1`))
  (`self.SyncSeatSound`))

(event `self.OnBrakelightToggled`
  (params (bEnabled :type Boolean)))

(event `CustomEvent_1`
  (params (Result :type "EAkResult Enum" :default "NotImplemented"))
  (if (or (`|EnumEquality` Result "BankAlreadyLoaded") (`|EnumEquality` Result "Success"))
    (`/Engine/EditorBlueprintResources/StandardMacros.DoOnce` false
      (:`Completed`
        (`AkComponent.SetOutputBusVolume` (`self.EngineSound`) 0.0)
        (`AkComponent.SetOutputBusVolume` (`self.RotorSound`) 0.0)
        (`AkComponent.SetOutputBusVolume` (`self.TurbineSound`) 0.0)
        (`AkGameObject.PostAssociatedAkEvent` :`self` (`self.TurbineSound`))
        (`AkGameObject.PostAssociatedAkEvent` :`self` (`self.EngineSound`))
        (`AkGameObject.PostAssociatedAkEvent` :`self` (`self.RotorSound`))
        (`KismetSystemLibrary.Delay` 0.1)
        (`self.SyncSeatSound`)))))

(event `self.EnginePart.Delegate_OnPartDamaged`
  (params (VehiclePart :type "VehiclePartComponent Object Reference") (Damage :type "Float (single-precision)"))
  (if (<= (`VehiclePartComponent.Health` VehiclePart) (* (`VehiclePartComponent.MaxHealth` VehiclePart) 0.25))
    (`/Engine/EditorBlueprintResources/StandardMacros.DoOnce` false
      (:`Completed`
        (`self.ToggleEngineStatus` false)))))

(event `self.ReceiveDestroyed`
  (`AkGameObject.Stop` (`self.EngineSound`))
  (`AkGameObject.Stop` (`self.RotorSound`))
  (`AkGameObject.Stop` (`self.TurbineSound`)))

(fn `SyncSeatSound`
  (locals (inseat1 :type Boolean))
  (bind _inseat1 (`local.inseat1`))
  (bind _turbinesound (`self.TurbineSound`))
  (bind _returnvalue (`Controller.K2_GetPawn` (`GameplayStatics.GetPlayerController` 0)))
  (if (`KismetSystemLibrary.IsValid` _returnvalue)
    (set `local.inseat1` false)
    (for _array_element (`self.GetSeatComponents`)
      (bind _returnvalue_2 (`VehicleSeatComponent.GetSeatedCharacter` _array_element))
      (if (`KismetSystemLibrary.IsValid` _returnvalue_2)
        (if (== _returnvalue _returnvalue_2)
          (set `local.inseat1` true)
          (break)))))
  (`AkComponent.SetRTPCValue` _turbinesound null (select `bool` _inseat1 :`true` 1.0 :!type "Float (single-precision)") 0 "RTPC_VehicleInOut")
  (`AkComponent.SetOutputBusVolume` _turbinesound (select `bool` _inseat1 :`false` 1.0 :`true` 0.5 :!type "Float (single-precision)"))
  (`AkComponent.SetOutputBusVolume` (`self.EngineSound`) (select `bool` _inseat1 :`false` 0.5 :!type "Float (single-precision)"))
  (`AkComponent.SetOutputBusVolume` (`self.RotorSound`) (select `bool` _inseat1 :`false` 0.5 :!type "Float (single-precision)"))
  (return))

(fn `UserConstructionScript`)