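; Networked scissor lift that extends or retracts between configurable height indices when its activate dispatch fires, restoring its start state each round.
; The server steps through a montage array, multicasting each segment forward or in reverse on timed delays.
; After extending, it teleports players overlapping "stuck"-tagged components to random navmesh points near StuckTeleport.
; On start and round reset, it snaps the attached actor on buttonSocket_0 back to that socket.
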(event `OnRoundActive_Multicast`
  (bind _montages (`self.montages`))
  (bind _sm_electriclifter_02b_animated_polysurface47 (`self.SM_ElectricLifter_02b_animated_polySurface47`))
  ;[1 0.06244 0.07239] Set start states for server and for everyone on round start
  (if (`KismetSystemLibrary.IsServer`) :!label _label
    (set `self.inUse` false)
    (bind _output_get (set `self.isExtended` (`self.startExtended`)))
    (if _output_get
      (bind _output_get_2 (set `self.animState` (`KismetMathLibrary.Clamp` (`self.index_extended`) 0 9)))
      (bind _output_get_3 (set `self.SyncIndex` _output_get_2))
      (`KismetSystemLibrary.Delay` 0.5 :!label _label_2)
      (`|PlayMontage` _sm_electriclifter_02b_animated_polysurface47 (`|GetArrayItem` _montages _output_get_3) 100.0 0.454 "Default"
        (:`then`
          _))
      (else
        (bind _output_get_4 (set `self.animState` (`KismetMathLibrary.Clamp` (`self.index_retracted`) 0 9)))
        (bind _output_get_5 (set `self.SyncIndex` _output_get_4))
        (`KismetSystemLibrary.Delay` 0.5 :!label _label_3)
        (`|PlayMontage` _sm_electriclifter_02b_animated_polysurface47 (`|GetArrayItem` _montages _output_get_5) 0.0 0.0 "Default"
          (:`then`
            _))))
    (elif (`self.startExtended`)
      (goto _label_2)
      (else
        (goto _label_3))))
  (`KismetSystemLibrary.Delay` 1.0)
  (`self.Func_SyncFirstPlatformSocketActor`))

(event `self.ReceiveBeginPlay`
  (`SkeletalMeshComponent.SetAnimationMode` (`self.SM_ElectricLifter_02b_animated_polySurface47`) "AnimationBlueprint")
  (`|ExecutionSequence`
    (:`then_0`
      (if (`KismetSystemLibrary.IsServer`)
        (`|ExecutionSequence`
          (:`then_0`
            (goto _label))
          (:`then_1`
            ;[1 0.2629 0.07239] Server start binds
            (add `self.Activate_Dispatch` (delegate `Activate_Dispatch_Event`)))
          (:`then_2`
            (bind _asinsmultiplayer_mode (cast `INSMultiplayerMode` (`GameplayStatics.GetGameMode`)))
            (add `INSMultiplayerMode.OnRoundActiveDelegate` _asinsmultiplayer_mode (delegate `ONROUNDACTIVE`))))))
    (:`then_1`
      ;[0.1255 1 0.8195] Client_start_state
      (`KismetSystemLibrary.Delay` 0.1)
      (if (not (`KismetSystemLibrary.IsServer`))
        (`|PlayMontage` (`self.SM_ElectricLifter_02b_animated_polySurface47`) (`|GetArrayItem` (`self.montages`) (`self.SyncIndex`)) (`KismetMathLibrary.SelectFloat` 100.0 0.0 (`self.isExtended`)) 0.0 "Default")))
    (:`then_2`
      (`self.Func_SyncFirstPlatformSocketActor`))))

(event `ONROUNDACTIVE`
  ;[1 0.2629 0.07239] Server start binds
  (`self.OnroundACtive_MUlticast`))

(event `ResetSound`
  ;[1 0.2891 0.7021] CreakySound
  (goto _label_4 :!via `Reset`))

(event `MulticastActivate`
  (bind _animstate (`self.animState`))
  (bind _output (`|GetArrayItem` (`self.montages`) (`self.animState`)))
  ;[0.5373 0.5608 0.1412] Animation Loop
  (`|ExecutionSequence`
    (:`then_0`
      ;[1 0.2891 0.7021] CreakySound
      (`/Engine/EditorBlueprintResources/StandardMacros.DoOnce` false :!label _label_4
        (:`Completed`
          (`AkGameplayStatics.PostEvent` "/Game/Audio/wwise/Sandstorm/Physics/Dynamic_Props/Doors/Reinforced/Movement/Play_ReinforcedDoor_Open_Creak.Play_ReinforcedDoor_Open_Creak" self))))
    (:`then_1`
      (set `self.SyncIndex` (`self.animState`))
      (`|PlayMontage` (`self.SM_ElectricLifter_02b_animated_polySurface47`) _output (* (`self.currentRateMult`) (`self.speedMultiplier`)) 0.0 "Default"
        (:`then`
          (if (`KismetSystemLibrary.IsServer`)
            (`KismetSystemLibrary.Delay` (/ (`AnimSequenceBase.SequenceLength` _output) (`self.speedMultiplier`)))
            (if (`self.isExtended`)
              ;[1 0.3827 0] Retraction
              (set `self.animState` (- _animstate 1))
              (if (!= _animstate (- (`KismetMathLibrary.Clamp` (`self.index_retracted`) 0 9) 1))
                ;[0.5373 0.5608 0.1412] Loop
                (`self.MulticastActivate` :!label _label_5)
                (else
                  ;[0.2511 0.7552 0.003738] Extension
                  (bind _output_get (set `self.isExtended` (not (`self.isExtended`)) :!label _label_6))
                  (set `self.inUse` false)
                  ;[0.1562 0.5953 1] Stuck Prevention
                  (`|ExecutionSequence`
                    (:`then_0`
                      (`self.Done_Dispatch`)
                      (`self.ResetSound`))
                    (:`then_1`
                      (if _output_get
                        (bind _outactors (`GameplayStatics.GetAllActorsOfClass` "/Script/NavigationSystem.RecastNavMesh"))
                        ;;[0 0.1344 1] Any primitive components tagged 'stuck' can be used for this
                        (for _array_element (`SceneComponent.GetChildrenComponents` (`self.SM_ElectricLifter_02b_animated_polySurface47`) true)
                          (if (`ActorComponent.ComponentHasTag` _array_element "stuck")
                            (bind _asprimitive_component (cast `PrimitiveComponent` _array_element))
                            (for _array_element_2 (`PrimitiveComponent.GetOverlappingActors` _asprimitive_component "/Game/Game/Actors/Characters/BP_Character_Player.BP_Character_Player_C")
                              (`self.K2_SetActorLocation` _array_element_2 (+ (`NavigationSystemV1.K2_GetRandomReachablePointInRadius` (`SceneComponent.K2_GetComponentLocation` (`self.Stuck_Teleport`)) (`SphereComponent.GetScaledSphereRadius` (`self.Stuck_FindRadius`)) (`|GetArrayItem` _outactors) null) (0.0 0.0 60.0)) false true))))))
                    (:`then_2`
                      (`self.Done_Dispatch`)))))
              (else
                (set `self.animState` (+ _animstate 1))
                (if (!= _animstate (+ (`KismetMathLibrary.Clamp` (`self.index_extended`) 0 9) 1))
                  (goto _label_5)
                  (else
                    (goto _label_6)))))))))))

(event `Activate_Dispatch_Event`
  ;[0.3125 0.02367 0.2645] Call Elevator
  (if (and (`KismetSystemLibrary.IsServer`) (not (`self.inUse`)))
    (set `self.inUse` true)
    (if (`self.isExtended`)
      (set `self.currentRateMult` -1.0)
      (set `self.animState` (`KismetMathLibrary.Clamp` (`self.index_extended`) 0 9))
      (else
        (set `self.currentRateMult` 1.0)
        (set `self.animState` (`KismetMathLibrary.Clamp` (`self.index_retracted`) 0 9))))
    (`self.MulticastActivate`)
    (`self.Done_Dispatch`)))

(fn `Func_SyncFirstPlatformSocketActor`
  (for _array_element (`self.GetAttachedActors` self true)
    (if (== (`self.GetAttachParentSocketName` _array_element) "buttonSocket_0")
      (`self.K2_SetActorLocation` _array_element (`SceneComponent.GetSocketLocation` (`self.SM_ElectricLifter_02b_animated_polySurface47`) "buttonSocket_0") false false)
      (break)))
  (return))

(fn `UserConstructionScript`
  (bind _sm_electriclifter_02b_animated_polysurface47 (`self.SM_ElectricLifter_02b_animated_polySurface47`))
  (if (`self.startExtended`)
    (set `SkeletalMeshComponent.AnimationData` (make `SingleAnimationPlayData` (`|GetArrayItem` (`self.montages`) (`KismetMathLibrary.Clamp` (`self.index_extended`) 0 9)) false false 0.454) _sm_electriclifter_02b_animated_polysurface47)
    (else
      (set `SkeletalMeshComponent.AnimationData` (make `SingleAnimationPlayData` (`|GetArrayItem` (`self.montages`) (`KismetMathLibrary.Clamp` (`self.index_retracted`) 0 9)) false false) _sm_electriclifter_02b_animated_polysurface47))))