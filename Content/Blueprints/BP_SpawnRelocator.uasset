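; Trigger volume that relocates freshly spawned AI player characters to a target location while its linked objective is under counter-attack.
; After a short BeginPlay delay it binds to the counter objective's owner-change and active-state delegates, switching on when a counter-attack objective changes owner and off when it deactivates.
; Overlapping AI created within the last few seconds are teleported to a random offset around the target, with SetActorLocation as fallback.
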(event `self.Box.OnComponentBeginOverlap`
  (params (OverlappedComponent :type "PrimitiveComponent Object Reference") (OtherActor :type "Actor Object Reference") (OtherComp :type "PrimitiveComponent Object Reference") (OtherBodyIndex :type Integer) (bFromSweep :type Boolean) (SweepResult :type "HitResult Structure (by ref)"))
  (bind _returnvalue (+ (`self.K2_GetActorLocation` (`|ConvertAsset` (`self.Target`))) (`KismetMathLibrary.MakeVector` (`KismetMathLibrary.RandomFloatInRange` -400.0 400.0) (`KismetMathLibrary.RandomFloatInRange` -400.0 400.0) (`KismetMathLibrary.RandomFloatInRange` 120.0 70.0))))
  (if (`self.active`)
    (bind _asbp_character_player (cast `/Game/Game/Actors/Characters/BP_Character_Player` OtherActor))
    (if (`INSCharacter.IsAIControlled` _asbp_character_player)
      (bind _returnvalue_2 (`self.GetGameTimeSinceCreation` _asbp_character_player))
      (if (< _returnvalue_2 5.0)
        (bind _returnvalue_3 (`self.K2_TeleportTo` :`self` OtherActor :`DestLocation` _returnvalue))
        (if (not _returnvalue_3)
          (`self.K2_SetActorLocation` OtherActor _returnvalue false false))
        (else
          (`KismetSystemLibrary.PrintString` (`KismetStringLibrary.Conv_DoubleToString` _returnvalue_2)))))))

(event `self.ReceiveBeginPlay`
  (bind _output (`|ConvertAsset` (`self.CounterObjective`)))
  (`KismetSystemLibrary.Delay` 1.0)
  (if (and (`KismetSystemLibrary.IsValid` _output) (`KismetSystemLibrary.IsValid` (`|ConvertAsset` (`self.Target`))))
    (add `ObjectiveBase.OnObjectiveChangeOwnerDelegate` _output (delegate `CustomEvent_0`))
    (add `ObjectiveBase.OnObjectiveActiveDelegate` _output (delegate `CustomEvent_1`))))

(event `CustomEvent_0`
  (params (Objective :type "ObjectiveBase Object Reference") (NewOwners :type Byte))
  (if (`ObjectiveBase.bCounterAttack` Objective)
    (set `self.active` true)))

(event `CustomEvent_1`
  (params (bNewActiveState :type Boolean) (Objective :type "ObjectiveBase Object Reference"))
  (if (not bNewActiveState)
    (set `self.active` false)))

(fn `UserConstructionScript`)